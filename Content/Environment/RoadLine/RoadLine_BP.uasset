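; RoadLine_BP is an environment actor that draws a colored road line along an editable spline.
; Its construction script loops over the spline point indices, adding a spline mesh component for each and matching start and end positions and tangents to consecutive points in local space.
; Each mesh gets a dynamic material instance driven by the Speed and Color variables, with Speed feeding the "u" parameter.
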(fn `UserConstructionScript`
  (bind _spline (`self.Spline`))
  (for _index (range (+ (`SplineComponent.GetNumberOfSplinePoints` _spline) 1))
    (bind _returnvalue (`AddComponent|NODE_AddSplineMeshComponent-0`))
    (bind _returnvalue_2 (+ _index 1))
    (`SplineMeshComponent.SetStartAndEnd` _returnvalue (`SplineComponent.GetLocationAtSplinePoint` _spline _index "Local") (`SplineComponent.GetTangentAtSplinePoint` _spline _index "Local") (`SplineComponent.GetLocationAtSplinePoint` _spline _returnvalue_2 "Local") (`SplineComponent.GetTangentAtSplinePoint` _spline _returnvalue_2 "Local") true)
    (bind _returnvalue_3 (`PrimitiveComponent.CreateDynamicMaterialInstance` _returnvalue 0 null "None"))
    (`MaterialInstanceDynamic.SetScalarParameterValue` _returnvalue_3 "u" (`self.Speed`))
    (`MaterialInstanceDynamic.SetVectorParameterValue` _returnvalue_3 "color" (`self.Color`))))