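; Spline actor that drips rainwater along its length, driven by the Ultra Dynamic Weather parameter collection.
; It samples points along the spline and line-traces down from each, passing positions and death heights to Niagara arrays as precomputed collision, optionally refreshed every tick.
; Rain and wetness scale the length-based spawn rate, rain drives splash duplication and wind drives curl noise.
; Tick starts after a random delay at BeginPlay.
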(event `/Visualization/Environment/Sky/Blueprints/Weather_Effects/Weather_Effects_Interface.Editor Update`
  (`self.Update with Weather`))

(event `self.ReceiveBeginPlay`
  (set `self.Runtime` true)
  (`self.Create Curve Data`)
  (`KismetSystemLibrary.Delay` (`KismetMathLibrary.RandomFloatInRange` 0.0 3.0))
  (`self.SetActorTickEnabled` true))

(event `self.ReceiveTick`
  (params (DeltaSeconds :type "Float (single-precision)"))
  (`self.Update with Weather`)
  (if (`self.Update Collision Regularly`)
    (`self.Create Curve Data`)))

(event `/Visualization/Environment/Sky/Blueprints/Weather_Effects/Weather_Effects_Interface.Reset Emitters`
  (`KismetSystemLibrary.Delay` 0.05)
  (`self.Update with Weather`)
  (`NiagaraComponent.ReinitializeSystem` (`self.Dripping_Curve`)))

(fn `Create Curve Data`
  (locals (Total_Distance :type "Float (double-precision)" :default 0.0) (`Last Collision Index` :type Integer :default 0))
  (set `local.Total_Distance` (`SplineComponent.GetSplineLength` (`self.Spline`)))
  (`KismetArrayLibrary.Array_Clear` (`self.Death Heights Array`))
  (`KismetArrayLibrary.Array_Clear` (`self.Positions Array`))
  (bind _output_get (set `local.Last Collision Index` (`KismetMathLibrary.Clamp` (`KismetMathLibrary.FCeil` (/ (`local.Total_Distance`) (`self.Point Spacing`))) 1 1000)))
  (for _index (range (+ _output_get 1))
    (bind _returnvalue (`SplineComponent.GetLocationAtDistanceAlongSpline` (`self.Spline`) (`KismetMathLibrary.MapRangeClamped` (`KismetMathLibrary.Conv_IntToDouble` _index) 0.0 (`KismetMathLibrary.Conv_IntToDouble` (`local.Last Collision Index`)) 0.0 (`local.Total_Distance`)) "World"))
    (`KismetArrayLibrary.Array_Add` (`self.Positions Array`) _returnvalue)
    (bind _returnvalue_2 (- _returnvalue (0.0 0.0 10000.0)))
    (bind (_outhit _returnvalue_3) (`KismetSystemLibrary.LineTraceSingle` (- _returnvalue (`KismetMathLibrary.MakeVector` 0.0 0.0 (`self.Collision Line Trace Head Start`))) _returnvalue_2 (`self.Collision Trace Channel`) false (`self.Collision Actors to Ignore`) (select `bool` (`self.Runtime`) :`false` "ForDuration" :!type "EDrawDebugTrace Enum") true (struct :`R` 0.194618 :`G` 0.327778 :`B` 0.462077 :`A` 1.0) (struct :`A` 1.0) 0.1))
    (if _returnvalue_3
      (`KismetArrayLibrary.Array_Add` (`self.Death Heights Array`) (.z (`.Location` (`GameplayStatics.BreakHitResult` _outhit))))
      (else
        (`KismetArrayLibrary.Array_Add` (`self.Death Heights Array`) (.z _returnvalue_2)))))
  (`NiagaraDataInterfaceArrayFunctionLibrary.SetNiagaraArrayFloat` (`self.Dripping_Curve`) "Death Heights" (`self.Death Heights Array`))
  (`FXSystemComponent.SetFloatParameter` (`self.Dripping_Curve`) "Collision Frequency" (`self.Point Spacing`))
  (`NiagaraDataInterfaceArrayFunctionLibrary.SetNiagaraArrayVector` (`self.Dripping_Curve`) "Positions Along Curve" (`self.Positions Array`)))

(fn `Update with Weather`
  (locals (Raining :type "Float (double-precision)" :default 0.0))
  (bind _returnvalue (`KismetMaterialLibrary.GetScalarParameterValue` "/Visualization/Environment/Sky/Materials/Weather/UltraDynamicWeather_Parameters.UltraDynamicWeather_Parameters" "Wet"))
  (bind _returnvalue_2 (`KismetMaterialLibrary.GetScalarParameterValue` "/Visualization/Environment/Sky/Materials/Weather/UltraDynamicWeather_Parameters.UltraDynamicWeather_Parameters" "Raining"))
  (set `local.Raining` _returnvalue_2)
  (`FXSystemComponent.SetFloatParameter` (`self.Dripping_Curve`) "Spawn Rate" (* (`KismetMathLibrary.FClamp` (+ _returnvalue_2 (* _returnvalue 0.01))) (+ (* (`self.Spawn Rate Per Meter`) (/ (`SplineComponent.GetSplineLength` (`self.Spline`)) 100.0)) (`self.Additional Spawn Rate`))))
  (bind _returnvalue_3 (`KismetMaterialLibrary.GetVectorParameterValue` "/Visualization/Environment/Sky/Materials/Weather/UltraDynamicWeather_Parameters.UltraDynamicWeather_Parameters" "Wind Force"))
  (`FXSystemComponent.SetFloatParameter` (`self.Dripping_Curve`) "Curl Noise Force" (* (`KismetMathLibrary.MapRangeClamped` (`KismetMathLibrary.VSize` (`KismetMathLibrary.Conv_LinearColorToVector` _returnvalue_3)) 0.0 2000.0 42.0 140.0) (`self.Curl Noise Force`)))
  (`FXSystemComponent.SetIntParameter` (`self.Dripping_Curve`) "Splash Duplicate Count" (`KismetMathLibrary.Round` (`KismetMathLibrary.MapRangeClamped` (`local.Raining`) 0.1 1.0 1.0 2.0)))
  (`FXSystemComponent.SetFloatParameter` (`self.Dripping_Curve`) "Splash Duplicate Range" (`KismetMathLibrary.MapRangeClamped` (`local.Raining`) 0.0 1.0 0.0 6.0)))

(fn `UserConstructionScript`
  (set `self.Refresh` false)
  (`self.Create Curve Data`)
  (`self.Update with Weather`)
  (`FXSystemComponent.SetFloatParameter` (`self.Dripping_Curve`) "Splash Percentage" (`self.Splash Frequency`))
  (`FXSystemComponent.SetFloatParameter` (`self.Dripping_Curve`) "Drop Scale" (`self.Drops Scale`)))