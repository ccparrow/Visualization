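; Spline-based road Blueprint that builds itself in the construction script by laying copies of a static mesh along its spline.
; The segment count is spline length divided by the mesh's scaled bounding-box max X, rounded to nearest with a minimum of one.
; Each spline mesh component spans an equal length, so segments stretch to fit exactly.
; Endpoints are shifted by an offset in spline space, with tangents scaled to segment length.
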(fn `AddMesh`
  (locals (_Number :type Integer) (_Length :type "Float (double-precision)" :default 0.0))
  (bind (_scale_x _scale_y) (`KismetMathLibrary.BreakVector` (`self.Scale`)))
  (bind _spline (`self.Spline`))
  (bind _scale_x_2 (`KismetMathLibrary.BreakVector` (`self.Scale`)))
  (bind _returnvalue (* (.x (`.Max` (break `Box` (`StaticMesh.GetBoundingBox` (`self.StaticMesh`))))) _scale_x_2))
  (bind (_remainder _returnvalue_2) (`KismetMathLibrary.FMod` (`SplineComponent.GetSplineLength` (`self.Spline`)) _returnvalue))
  ;[1 1 1] 模型段数
  (set `local._Number` (select `bool` (>= _remainder (* _returnvalue 0.5)) :`false` (`KismetMathLibrary.Max` _returnvalue_2 1) :`true` (+ _returnvalue_2 1)))
  ;[1 1 1] 单位长度
  (set `local._Length` (/ (`SplineComponent.GetSplineLength` (`self.Spline`)) (`KismetMathLibrary.Conv_IntToDouble` (`local._Number`))))
  (for _index (range (`local._Number`))
    (bind _returnvalue_3 (`AddComponent|NODE_AddSplineMeshComponent-3` :`RelativeTransform` (`KismetMathLibrary.MakeTransform` (0.0 0.0 0.0) (struct) (`self.Scale`))))
    (`StaticMeshComponent.SetStaticMesh` _returnvalue_3 (`self.StaticMesh`))
    (`SplineMeshComponent.SetStartScale` _returnvalue_3 (`KismetMathLibrary.MakeVector2D` _scale_x _scale_y) true)
    (`SplineMeshComponent.SetEndScale` _returnvalue_3 (`KismetMathLibrary.MakeVector2D` _scale_x _scale_y) true)
    (bind _returnvalue_4 (* _index (`local._Length`)))
    (bind _returnvalue_5 (+ _returnvalue_4 (`local._Length`)))
    (`SplineMeshComponent.SetStartAndEnd` _returnvalue_3 (+ (`SplineComponent.GetLocationAtDistanceAlongSpline` _spline _returnvalue_4 "Local") (`KismetMathLibrary.TransformDirection` (`SplineComponent.GetTransformAtDistanceAlongSpline` _spline _returnvalue_4 "Local" true) (`self.Offset`))) (* (`SplineComponent.GetDirectionAtDistanceAlongSpline` _spline _returnvalue_4 "Local") (`local._Length`)) (+ (`SplineComponent.GetLocationAtDistanceAlongSpline` _spline _returnvalue_5 "Local") (`KismetMathLibrary.TransformDirection` (`SplineComponent.GetTransformAtDistanceAlongSpline` _spline _returnvalue_5 "Local" true) (`self.Offset`))) (* (`SplineComponent.GetDirectionAtDistanceAlongSpline` _spline _returnvalue_5 "Local") (`local._Length`)) true)))

(fn `UserConstructionScript`
  (locals (_Spline :type "SplineComponent Object Reference"))
  (`self.AddMesh`))