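; Street light actor that turns its spot light and lit lamp material on at night and off by day.
; On BeginPlay it binds to the night event dispatcher from VGIS, passing the night state to SwitchLight.
; The construction script runs the same function from the Night variable.
; A visibility event shows or hides the lamp mesh and always switches the light off.
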(event `self.ReceiveBeginPlay`
  (add `/Visualization/GamePlay/VGIS.Night_ED` (subsystem `/Visualization/GamePlay/VGIS`) (delegate `Night_ED_Event_0`)))

(event `Night_ED_Event_0`
  (params (bNight :type Boolean))
  (`self.SwitchLight` bNight))

(event `VisibilityLight_Event`
  (params (`Visibility?` :type Boolean))
  (`SceneComponent.SetVisibility` (`self.StreetLamp`) `Visibility?` false)
  (`self.SwitchLight` false))

(fn `SwitchLight`
  (params (bNight :type Boolean))
  (`PrimitiveComponent.SetMaterial` (`self.StreetLamp`) 1 (select `bool` bNight :`false` "/Visualization/Environment/StreetLight/Material/Light_Mat.Light_Mat" :`true` "/Visualization/Environment/StreetLight/Material/LightOn_Mat.LightOn_Mat" :!type "MaterialInterface Object Reference"))
  (`SceneComponent.SetVisibility` (`self.SpotLight`) bNight false))

(fn `UserConstructionScript`
  (`self.SwitchLight` (`self.bNight`)))