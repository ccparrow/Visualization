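; Car_TBP is an ambient traffic actor that loops a set of cars along a spline.
; Init adds randomly picked car meshes from a content folder, attaches light components at CarLight sockets, and spreads start times with Sobol randomness.
; Tick advances times at constant velocity, with Flip reversing direction, and wraps cars at the spline end.
; A construction-script Refresh toggle scales speed by spline length and previews placement; Night and Anim events toggle light and car visibility.
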(event `self.ReceiveBeginPlay`
  (`self.Init`) ; 设置汽车数量及Time值
  (add `/Visualization/GamePlay/VGIS.Night_ED` (subsystem `/Visualization/GamePlay/VGIS`) (`|CreateDelegate` :!event `Night_Event`)))

(event `self.ReceiveTick`
  (params (DeltaSeconds :type "Float (single-precision)"))
  ;[1 1 1] 汽车循环行驶
  (`self.Refresh`))

(event `Crystal_Event`
  (params (bCrystal :type Boolean))
  ;[1 1 1] 模式切换
)

(event `Night_Event`
  (params (bNight :type Boolean))
  ;[1 1 1] 模式切换
  (for _array_element (`self.CarLightArray`)
    (`SceneComponent.SetVisibility` _array_element bNight false)))

(event `Anim_Event`
  (params (bAnim :type Boolean))
  ;[1 1 1] 模式切换
  (for _array_element (`self.CarArray`)
    (`SceneComponent.SetVisibility` _array_element (not bAnim) false)))

(event `SetPointType`
  (bind _spline (`self.Spline`))
  ;[1 1 1] 改变样条线点的类型
  (for _index (range (`SplineComponent.GetNumberOfSplinePoints` _spline))
    (`SplineComponent.SetSplinePointType` _spline _index (`self.SplineType`) true)))

(fn `Init`
  (bind _carnumber (`self.CarNumber`))
  (bind _distanceseed (`self.DistanceSeed`))
  (bind _scale (`self.Scale`))
  (`KismetArrayLibrary.Array_Clear` (`self.TimeArray`))
  (for _index (range _carnumber)
    (`KismetArrayLibrary.Array_Add` (`self.TimeArray`) (+ (`ImportanceSamplingLibrary.RandomSobolFloat` _index _carnumber (`KismetMathLibrary.RandomFloatInRange` (- 0.5 _distanceseed) (+ 0.5 _distanceseed))) (`self.AddDistance`)))
    (bind _returnvalue (`AddComponent|NODE_AddStaticMeshComponent-0` :`RelativeTransform` (`KismetMathLibrary.MakeTransform` (0.0 0.0 0.0) (struct) _scale)))
    (`KismetArrayLibrary.Array_Add` (`self.CarArray`) _returnvalue)
    (bind _asstatic_mesh (`self.RandomMesh`))
    (`StaticMeshComponent.SetStaticMesh` _returnvalue _asstatic_mesh)
    (bind _returnvalue_2 (`AddComponent|NODE_AddStaticMeshComponent-1` :`RelativeTransform` (`KismetMathLibrary.MakeTransform` (0.0 0.0 0.0) (struct) _scale)))
    (`SceneComponent.K2_AttachToComponent` _returnvalue_2 _returnvalue "CarLight" "SnapToTarget" "SnapToTarget" "SnapToTarget" true)
    (`KismetArrayLibrary.Array_Add` (`self.CarLightArray`) _returnvalue_2)))

(fn `RandomMesh`
  (returns (`AsStatic Mesh` :type "StaticMesh Object Reference"))
  (bind _assetdataarray (`V_Library.LoadAssetDataFromDirectory` "/Visual/Environment/Car/Mesh"))
  (bind _asstatic_mesh (cast `StaticMesh` (`AssetRegistryHelpers.GetAsset` (`|GetArrayItem` _assetdataarray (`KismetMathLibrary.RandomIntegerFromStream` (- (`KismetArrayLibrary.Array_Length` _assetdataarray) 1) (`KismetMathLibrary.MakeRandomStream` (`KismetMathLibrary.RandomInteger` 99999)))))))
  (return _asstatic_mesh))

(fn `Refresh`
  (locals (_Index :type Integer))
  (bind _spline (`self.Spline`))
  (bind _spline_2 (`self.Spline`))
  (bind _returnvalue (* (`GameplayStatics.GetWorldDeltaSeconds`) (`self._SpeedRate`)))
  (bind _output (`|GetArrayItem` (`self.TimeArray`) (`local._Index`)))
  (bind _output_2 (`|GetArrayItem` (`self.TimeArray`) (`local._Index`)))
  (bind _returnvalue_2 (`SplineComponent.GetLocationAtTime` _spline _output "Local" true))
  (bind _returnvalue_3 (`KismetMathLibrary.Conv_VectorToRotator` (`SplineComponent.GetTangentAtTime` _spline _output "Local" true)))
  (for _index (range (`self.CarNumber`))
    (set `local._Index` _index)
    (`KismetArrayLibrary.Array_Set` (`self.TimeArray`) (`local._Index`) (select `bool` (`self.bFlip?`) :`false` (+ _output_2 _returnvalue) :`true` (- _output_2 _returnvalue))) ; 刷新Time值
    (`SceneComponent.K2_SetRelativeLocationAndRotation` (`|GetArrayItem` (`self.CarArray`) (`local._Index`)) _returnvalue_2 (select `bool` (`self.bFlip?`) :`false` _returnvalue_3 :`true` (`KismetMathLibrary.MakeRotator` (.roll _returnvalue_3) (.pitch _returnvalue_3) (+ (.yaw _returnvalue_3) 180.0))) false false) ; 刷新汽车位置
    (if (== (`SplineComponent.GetLocationAtSplinePoint` _spline_2 (select `bool` (`self.bFlip?`) :`false` (- (`SplineComponent.GetNumberOfSplinePoints` _spline_2) 1)) "Local") _returnvalue_2 :`ErrorTolerance` 50.0)
      (`KismetArrayLibrary.Array_Set` (`self.TimeArray`) (`local._Index`) (select `bool` (`self.bFlip?`) :`true` 1.0)) ; 重置Time值
    )))

(fn `SetSpepedRate`
  (set `self._SpeedRate` (/ (* (`self.SpeedRate`) 1500.0) (`SplineComponent.GetSplineLength` (`self.Spline`)))) ; 按长度拟合速率
)

(fn `UserConstructionScript`
  (if (`self.bRefresh`)
    (set `self.bRefresh` false)
    (`self.SetSpepedRate`) ; 速率拟合
    (`self.Init`) ; 设置汽车数量及Time值
    (`self.Refresh`) ; 改变汽车位置
  ))