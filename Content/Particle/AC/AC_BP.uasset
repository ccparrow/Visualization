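; AC_BP is an actor that feeds location and temperature data into a Niagara particle effect through array user parameters.
; The construction script copies its Locations and Temps variables into Temp_Locs and Temp_Values.
; BeginPlay then overwrites Temp_Locs with hardcoded test points and writes fixed values to a separate Flow_TempDeltas array, leaving Temp_Values untouched.
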(event `self.ReceiveBeginPlay`
  (bind _niagara (`self.Niagara`))
  (`NiagaraDataInterfaceArrayFunctionLibrary.SetNiagaraArrayVector` _niagara "Temp_Locs" (`|MakeArray` (0.0 0.0 0.0) (100.0 100.0 100.0) (-100.0 -100.0 0.0) :!type "Vector Structure"))
  (`NiagaraDataInterfaceArrayFunctionLibrary.SetNiagaraArrayFloat` _niagara "Flow_TempDeltas" (`|MakeArray` 60.0 10.0 20.0 :!type "Float (single-precision)")))

(fn `UserConstructionScript`
  (locals (Locations :type "Array of Vector Structure") (Temps :type "Array of Float (double-precision)"))
  (bind _niagara (`self.Niagara`))
  (`NiagaraDataInterfaceArrayFunctionLibrary.SetNiagaraArrayVector` _niagara "Temp_Locs" (`local.Locations`))
  (`NiagaraDataInterfaceArrayFunctionLibrary.SetNiagaraArrayFloat` _niagara "Temp_Values" (`local.Temps`)))