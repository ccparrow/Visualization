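; Sequence agent actor that starts and stops a level sequence on an animation event and reports it to pixel streaming through Visual_GameState.
; Starting focuses the player's Visual_Pawn on the actor's camera, unloads the Other_Map sublevel and plays the sequence.
; Stopping rewinds the sequence and reloads that sublevel.
; Helpers handle reverse play and normalized scrubbing, using a duration cached at BeginPlay.
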(event `self.ReceiveBeginPlay`
  (`self.GetMaxTime`))

(event `Animation_Event`
  (params (bAnim :type Boolean) (InfoID :type String))
  (bind _camera (`self.Camera`))
  (if bAnim
    (bind _asvisual_pawn (cast `/Visualization/GamePlay/Visual_Pawn` (`GameplayStatics.GetPlayerPawn` 0)))
    (`/Visualization/GamePlay/Visual_Pawn.FocusLocation_Event` _asvisual_pawn (`SceneComponent.K2_GetComponentLocation` _camera) (`SceneComponent.K2_GetComponentRotation` _camera) 0.0)
    (`GameplayStatics.UnloadStreamLevel` "Other_Map")
    (bind _asvisual_game_state (cast `/Visualization/GamePlay/Visual_GameState` (`GameplayStatics.GetGameState`)))
    (`/Visualization/GamePlay/Visual_GameState.SendPixelStreaming` _asvisual_game_state "" InfoID "animation" "3")
    (`self.PlaySequence`)
    (`KismetSystemLibrary.Delay` (`self.MaxTime`))
    (else
      (`self.SlideSequence` 0.0)
      (`self.StopSequence`)
      (bind _asvisual_game_state_2 (cast `/Visualization/GamePlay/Visual_GameState` (`GameplayStatics.GetGameState`)))
      (`/Visualization/GamePlay/Visual_GameState.SendPixelStreaming` _asvisual_game_state_2 "" InfoID "animation" "3")
      (`GameplayStatics.LoadStreamLevel` "Other_Map" true))))

(fn `GetMaxTime`
  (bind _sequenceref (`self.SequenceRef`))
  (bind (_frame _framerate) (`KismetMathLibrary.BreakQualifiedFrameTime` (`MovieSceneSequencePlayer.GetEndTime` (`LevelSequenceActor.SequencePlayer` _sequenceref))))
  (`/Engine/EditorBlueprintResources/StandardMacros.IsValid` _sequenceref
    (:`Is Valid`
      (set `self.MaxTime` (/ (`KismetMathLibrary.Conv_IntToDouble` (break `FrameNumber` _frame)) (`KismetMathLibrary.Conv_IntToDouble` (`KismetMathLibrary.BreakFrameRate` _framerate)))) ; 获得Sequence最大时间值
    )))

(fn `PlaySequence`
  (`MovieSceneSequencePlayer.Play` (`LevelSequenceActor.SequencePlayer` (`self.SequenceRef`))))

(fn `ReverseSequence`
  (`MovieSceneSequencePlayer.PlayReverse` (`LevelSequenceActor.SequencePlayer` (`self.SequenceRef`))))

(fn `SlideSequence`
  (params (SlideValue :type "Float (double-precision)"))
  (bind _maxtime (`self.MaxTime`))
  (`MovieSceneSequencePlayer.SetPlaybackPosition` (`LevelSequenceActor.SequencePlayer` (`self.SequenceRef`)) (make `MovieSceneSequencePlaybackParams` :`Time` (`KismetMathLibrary.FClamp` (* SlideValue _maxtime) 0.0 _maxtime))))

(fn `StopSequence`
  (`MovieSceneSequencePlayer.Stop` (`LevelSequenceActor.SequencePlayer` (`self.SequenceRef`))))

(fn `UserConstructionScript`
  (`SceneComponent.K2_SetRelativeTransform` (`self.Camera`) (`self.CameraTansform`) false false))