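; Base sequence actor that plays an embedded ActorSequence animation with its own camera, reporting to Pixel Streaming through Visual_GameState.
; Animation_Event either focuses Visual_Pawn on the camera, unloads Other_Map and plays, or resets the sequence and reloads that level.
; Helpers handle play, reverse, stop, normalized scrubbing via the MaxTime computed on BeginPlay, and child visibility.
; AnimFlip toggles forward and reverse playback using the Bloom flag.
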(event `Visibility_Event`
  (params (Target :type "SceneComponent Object Reference") (bNewVisibility :type Boolean) (bPropagateToChildren :type Boolean))
  (`SceneComponent.SetVisibility` Target bNewVisibility bPropagateToChildren))

(event `self.ReceiveBeginPlay`
  (`self.GetMaxTime`))

(event `Animation_Event`
  (params (bAnim :type Boolean) (InfoID :type String))
  (bind _camera (`self.Camera`))
  (if bAnim
    (bind _asvisual_pawn (cast `/Visualization/GamePlay/Visual_Pawn` (`GameplayStatics.GetPlayerPawn` 0)))
    (`/Visualization/GamePlay/Visual_Pawn.FocusLocation_Event` _asvisual_pawn (`SceneComponent.K2_GetComponentLocation` _camera) (`SceneComponent.K2_GetComponentRotation` _camera) 0.0)
    (`GameplayStatics.UnloadStreamLevel` "Other_Map")
    (bind _asvisual_game_state (cast `/Visualization/GamePlay/Visual_GameState` (`GameplayStatics.GetGameState`)))
    (`/Visualization/GamePlay/Visual_GameState.SendPixelStreaming` _asvisual_game_state "" InfoID "animation" "3")
    (`self.PlaySequence` 1.0)
    (`KismetSystemLibrary.Delay` (`self.MaxTime`))
    (else
      (`self.SlideSequence` 0.0)
      (`self.StopSequence`)
      (bind _asvisual_game_state_2 (cast `/Visualization/GamePlay/Visual_GameState` (`GameplayStatics.GetGameState`)))
      (`/Visualization/GamePlay/Visual_GameState.SendPixelStreaming` _asvisual_game_state_2 "" InfoID "animation" "3")
      (`GameplayStatics.LoadStreamLevel` "Other_Map" true))))

(fn `AnimFlip`
  (if (`self.bBloom`)
    (`self.ReverseSequence` 1.0)
    (set `self.bBloom` false)
    (else
      (`self.PlaySequence` 1.0)
      (set `self.bBloom` true))))

(fn `AnimInit`
  (`self.StopSequence`)
  (`self.SlideSequence` 0.0)
  (set `self.bBloom` false))

(fn `GetMaxTime`
  (bind (_frame _framerate) (`KismetMathLibrary.BreakQualifiedFrameTime` (`MovieSceneSequencePlayer.GetEndTime` (`ActorSequenceComponent.SequencePlayer` (`self.ActorSequence`)))))
  (set `self.MaxTime` (/ (`KismetMathLibrary.Conv_IntToDouble` (break `FrameNumber` _frame)) (`KismetMathLibrary.Conv_IntToDouble` (`KismetMathLibrary.BreakFrameRate` _framerate)))) ; 获得Sequence最大时间值
)

(fn `HiddenChildren_SF`
  (params (Target :type "SceneComponent Object Reference"))
  (`self.Visibility_Event` Target false true))

(fn `OnRep_bBloom`)

(fn `PlaySequence`
  (params (PlayRate :type "Float (double-precision)" :default 1.0) (NumLoops :type Integer :default 0))
  (bind _sequenceplayer (`ActorSequenceComponent.SequencePlayer` (`self.ActorSequence`)))
  (`MovieSceneSequencePlayer.Play` _sequenceplayer)
  (`MovieSceneSequencePlayer.SetPlayRate` _sequenceplayer PlayRate)
  (`MovieSceneSequencePlayer.PlayLooping` _sequenceplayer NumLoops))

(fn `ReverseSequence`
  (params (PlayRate :type "Float (double-precision)" :default 1.0) (NumLoops :type Integer))
  (bind _sequenceplayer (`ActorSequenceComponent.SequencePlayer` (`self.ActorSequence`)))
  (`MovieSceneSequencePlayer.PlayReverse` _sequenceplayer)
  (`MovieSceneSequencePlayer.SetPlayRate` _sequenceplayer PlayRate)
  (`MovieSceneSequencePlayer.PlayLooping` _sequenceplayer NumLoops))

(fn `SlideSequence`
  (params (SlideValue :type "Float (double-precision)"))
  (bind _maxtime (`self.MaxTime`))
  (`MovieSceneSequencePlayer.SetPlaybackPosition` (`ActorSequenceComponent.SequencePlayer` (`self.ActorSequence`)) (make `MovieSceneSequencePlaybackParams` :`Time` (`KismetMathLibrary.FClamp` (* SlideValue _maxtime) 0.0 _maxtime))))

(fn `StopSequence`
  (`MovieSceneSequencePlayer.Stop` (`ActorSequenceComponent.SequencePlayer` (`self.ActorSequence`))))

(fn `UserConstructionScript`
  (`self.AnimInit`)
  (`SceneComponent.K2_SetRelativeTransform` (`self.Camera`) (`self.CameraTansform`) false false))

(fn `VisibilityChildren_SF`
  (params (Target :type "SceneComponent Object Reference"))
  (`self.Visibility_Event` Target true true))