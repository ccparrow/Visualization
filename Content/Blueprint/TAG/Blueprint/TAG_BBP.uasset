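; Map tag actor that registers as a VGIS point of interest and shows a billboard and clickable text widget.
; A looping timer scales the widget down with 2D camera distance and hides it at minimum scale.
; Construction can aim the stored camera transform at the actor and adds an editor-only preview camera.
; Clicked focuses the Visual_Pawn on that view in editor, otherwise sends the tag ID through Pixel Streaming via Visual_GameState.
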(event `self.ReceiveBeginPlay`
  (bind _returnvalue (subsystem `/Visualization/GamePlay/VGIS`))
  ;[1 1 1] 开始同步instance
  (add `/Visualization/GamePlay/VGIS.Birdeye_ED` _returnvalue (`|CreateDelegate` :!event `Hidden`))
  (`KismetArrayLibrary.Array_Add` (`/Visualization/GamePlay/VGIS.POI` _returnvalue) self)
  ;[1 1 1] UI大小
  (`KismetSystemLibrary.K2_SetTimer` null "WidgetSize" 0.05 true)
  ;[1 1 1] UI
  (`self.WidgetInit`))

(event `self.ReceiveEndPlay`
  (params (EndPlayReason :type "EEndPlayReason Enum" :default "Destroyed"))
  ;[1 1 1] 结束清除instance
  (`KismetArrayLibrary.Array_RemoveItem` (`/Visualization/GamePlay/VGIS.POI` (subsystem `/Visualization/GamePlay/VGIS`)) self))

(fn `Clicked`
  (`V_Library.IsEditor`
    (:`Success`
      (`self.Focus` true))
    (:`Fail`
      (bind _asvisual_game_state (cast `/Visualization/GamePlay/Visual_GameState` (`GameplayStatics.GetGameState`)))
      (`/Visualization/GamePlay/Visual_GameState.SendPixelStreamingWithID` _asvisual_game_state (`V_Library.AddJsonString` "" "classify" "tag") "1234567" "click" "3" (`self.ID`)))))

(fn `Focus`
  (params (bFocus :type Boolean :default true))
  (bind _returnvalue (`self.GetTransform`))
  (bind _cameratransform (`self.CameraTransform`))
  (if bFocus
    (bind _asvisual_pawn (cast `/Visualization/GamePlay/Visual_Pawn` (`GameplayStatics.GetPlayerPawn` 0)))
    (`/Visualization/GamePlay/Visual_Pawn.FocusLocation_Event` _asvisual_pawn (+ (.location _returnvalue) (.location _cameratransform)) (`KismetMathLibrary.MakeRotator` (+ (.roll (.rotation _returnvalue)) (.roll (.rotation _cameratransform))) (+ (.pitch (.rotation _returnvalue)) (.pitch (.rotation _cameratransform))) (+ (.yaw (.rotation _returnvalue)) (.yaw (.rotation _cameratransform)))) (`self.ArmLength`))))

(fn `Hidden`
  (params (bHidden :type Boolean))
  (`SceneComponent.SetVisibility` (`self.Billboard`) (not bHidden) true))

(fn `UserConstructionScript`
  (bind _returnvalue (`self.K2_GetActorLocation`))
  (bind (_cameratransform_location _cameratransform_rotation) (`KismetMathLibrary.BreakTransform` (`self.CameraTransform`)))
  (bind _cameratransform_location_2 (`KismetMathLibrary.BreakTransform` (`self.CameraTransform`)))
  (if (`self.bCameraAimRoot`)
    (set `self.CameraTransform` (`KismetMathLibrary.MakeTransform` _cameratransform_location_2 (`KismetMathLibrary.FindLookAtRotation` (+ _cameratransform_location_2 _returnvalue) _returnvalue))))
  (`V_Library.IsEditor`
    (:`Success`
      (`AddComponent|NODE_AddCameraComponent-0` :`RelativeTransform` (`KismetMathLibrary.MakeTransform` _cameratransform_location _cameratransform_rotation)))
    (:`Fail`
      _))
  (`BillboardComponent.SetSprite` (`self.Billboard`) (`self.Texture`))
  (`SceneComponent.K2_SetRelativeLocation` (`self.Billboard`) (`KismetMathLibrary.MakeVector` 0.0 0.0 (`self.WidgetHight`)) false false))

(fn `WidgetInit`
  (bind _astag_wbp (cast `/Visualization/Blueprint/TAG/UMG/TAG_WBP` (`WidgetComponent.GetUserWidgetObject` (`self.Widget`))))
  (set `/Visualization/Blueprint/TAG/UMG/TAG_WBP.Text` (`self.Text`) _astag_wbp)
  (add `/Visualization/Blueprint/TAG/UMG/TAG_WBP.Clicked_ED` _astag_wbp (`|CreateDelegate` :!event `Clicked`)))

(fn `WidgetSize`
  (bind _widget (`self.Widget`))
  (bind _returnvalue (`SceneComponent.IsVisible` _widget))
  (bind _returnvalue_2 (`KismetMathLibrary.MapRangeClamped` (`KismetMathLibrary.Vector_Distance2D` (`PlayerCameraManager.GetCameraLocation` (`PlayerController.PlayerCameraManager` (`GameplayStatics.GetPlayerController` 0))) (`self.K2_GetActorLocation`)) 1000.0 10000.0 1.0 0.3))
  (bind _returnvalue_3 (<= _returnvalue_2 0.3))
  (`Widget.SetRenderScale` (`WidgetComponent.GetUserWidgetObject` (`self.Widget`)) (`KismetMathLibrary.MakeVector2D` _returnvalue_2 _returnvalue_2))
  (if _returnvalue_3
    (if _returnvalue
      (`SceneComponent.SetVisibility` _widget (not _returnvalue_3) false :!label _label))
    (elif (not _returnvalue)
      (goto _label))))