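; IOT tag actor that shows a clickable IOT_WBP widget at a world location.
; WidgetInit passes the texture to the widget and binds its click delegate.
; WidgetSize shrinks the widget with 2D camera distance and hides it at minimum scale.
; Clicked focuses when the IsEditor check succeeds, otherwise sends an "iot" click message with the tag's ID over Pixel Streaming through Visual_GameState.
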(fn `Clicked`
  (`V_Library.IsEditor`
    (:`Success`
      (`self.Focus` true))
    (:`Fail`
      (bind _asvisual_game_state (cast `/Visualization/GamePlay/Visual_GameState` (`GameplayStatics.GetGameState`)))
      (`/Visualization/GamePlay/Visual_GameState.SendPixelStreamingWithID` _asvisual_game_state (`V_Library.AddJsonString` "" "classify" "iot") "1234567" "click" "3" (`self.ID`)))))

(fn `UserConstructionScript`
  (`parent.UserConstructionScript`))

(fn `WidgetInit`
  (bind _asiot_wbp (cast `/Visualization/Blueprint/TAG/UMG/IOT_WBP` (`WidgetComponent.GetUserWidgetObject` (`self.Widget`))))
  (set `/Visualization/Blueprint/TAG/UMG/IOT_WBP.Texture` (`self.Texture`) _asiot_wbp)
  (add `/Visualization/Blueprint/TAG/UMG/IOT_WBP.Clicked_ED` _asiot_wbp (`|CreateDelegate` :!event `Clicked`)))

(fn `WidgetSize`
  (bind _widget (`self.Widget`))
  (bind _returnvalue (`SceneComponent.IsVisible` _widget))
  (bind _returnvalue_2 (`KismetMathLibrary.MapRangeClamped` (`KismetMathLibrary.Vector_Distance2D` (`PlayerCameraManager.GetCameraLocation` (`PlayerController.PlayerCameraManager` (`GameplayStatics.GetPlayerController` 0))) (`self.K2_GetActorLocation`)) 1000.0 10000.0 1.0 0.3))
  (bind _returnvalue_3 (<= _returnvalue_2 0.3))
  (`Widget.SetRenderScale` (`WidgetComponent.GetUserWidgetObject` (`self.Widget`)) (`KismetMathLibrary.MakeVector2D` _returnvalue_2 _returnvalue_2))
  (if _returnvalue_3
    (if _returnvalue
      (`SceneComponent.SetVisibility` _widget (not _returnvalue_3) false :!label _label))
    (elif (not _returnvalue)
      (goto _label))))