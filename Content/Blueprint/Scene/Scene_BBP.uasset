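; Scene Blueprint that toggles a self-contained view, hidden at BeginPlay, which the player is moved into and back out of via Scene_Event.
; Entering shows the root hierarchy and post process, saves the pawn's location, control rotation and Visual_Pawn camera arm settings, then moves the pawn above the actor, facing the Arrow, with FixPawn enabled and this scene's arm limits.
; Leaving restores the saved state and hides the scene again.
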(event `self.ReceiveBeginPlay`
  (`self.SetVisibility` false) ; 隐藏场景
)

(event `Scene_Event`
  (params (bScene :type Boolean))
  (if bScene
    (`self.InScene`)
    (else
      (`self.OutScene`))))

(fn `InScene`
  (`self.SetVisibility` true) ; 显示场景
  (set `self._LocationSave` (`self.K2_GetActorLocation` (`GameplayStatics.GetPlayerPawn` 0))) ; 保存位置
  (set `self._RotationSave` (`Controller.GetControlRotation` (`GameplayStatics.GetPlayerController` 0))) ; 保存旋转
  (`self.K2_SetActorLocation` (`GameplayStatics.GetPlayerPawn` 0) (+ (`self.K2_GetActorLocation`) (`KismetMathLibrary.MakeVector` 0.0 0.0 (`self.AddZ`))) false false)
  (`Controller.SetControlRotation` (`GameplayStatics.GetPlayerController` 0) (`KismetMathLibrary.MakeRotator` 0.0 (.pitch (`SceneComponent.K2_GetComponentRotation` (`self.Arrow`))) (.yaw (`SceneComponent.K2_GetComponentRotation` (`self.Arrow`)))))
  (bind _asvisual_pawn (cast `/Visualization/GamePlay/Visual_Pawn` (`GameplayStatics.GetPlayerPawn` 0)))
  (bind (_bfixpawn _armlength _armlengthmin _armlengthmax) (`/Visualization/GamePlay/Visual_Pawn.GetFixPawn` _asvisual_pawn))
  (set `self._FixSave` _bfixpawn)
  (set `self._ArmLengthSave` _armlength)
  (set `self._ArmMinSave` _armlengthmin)
  (set `self._ArmMaxSave` _armlengthmax)
  (`/Visualization/GamePlay/Visual_Pawn.SetFixPawn` _asvisual_pawn true (`self.ArmLength`) (`self.ArmMin`) (`self.ArmMax`)))

(fn `OutScene`
  (`self.K2_SetActorLocation` (`GameplayStatics.GetPlayerPawn` 0) (`self._LocationSave`) false true) ; 恢复位置
  (`Controller.SetControlRotation` (`GameplayStatics.GetPlayerController` 0) (`self._RotationSave`)) ; 恢复旋转
  (bind _asvisual_pawn (cast `/Visualization/GamePlay/Visual_Pawn` (`GameplayStatics.GetPlayerPawn` 0)))
  (`/Visualization/GamePlay/Visual_Pawn.SetFixPawn` _asvisual_pawn (`self._FixSave`) (`self._ArmLengthSave`) (`self._ArmMinSave`) (`self._ArmMaxSave`))
  (`self.SetVisibility` false) ; 隐藏场景
)

(fn `SetVisibility`
  (params (bVisibility :type Boolean))
  (bind _root (`self.Root`))
  (`SceneComponent.SetVisibility` _root bVisibility true)
  (`SceneComponent.SetHiddenInGame` _root (not bVisibility) true)
  (set `PostProcessComponent.bEnabled` bVisibility (`self.PostProcess`))
  (`SceneComponent.SetHiddenInGame` (`self.Arrow`) true false))

(fn `UserConstructionScript`
  (`self.SetVisibility` (`self.bVisibility`)))