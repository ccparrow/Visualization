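; A test actor that controls an external AirRaidShelter packaged executable from keyboard input.
; On BeginPlay it enables input for the first player controller.
; Key 1 launches the exe from a hardcoded path with offscreen rendering, key 2 checks whether it runs, and key 3 closes it by name.
; Launch and status results are printed on screen.
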(event `self.ReceiveBeginPlay`
  (`self.EnableInput` (`GameplayStatics.GetPlayerController` 0)))

(event `Key|One`
  (params (Key :type "Key Structure"))
  (:`Pressed`
    (bind _returnvalue (`self.createProcess` "D:\\Package\\AirRaidShelter\\WindowsNoEditor\\AirRaidShelter.exe" "-renderoffscreen"))
    (`KismetSystemLibrary.PrintString` (`KismetStringLibrary.Conv_BoolToString` _returnvalue) true true (struct :`G` 0.66 :`B` 1.0 :`A` 1.0) 10.0)))

(event `Key|Two`
  (params (Key :type "Key Structure"))
  (:`Pressed`
    (bind _returnvalue (`self.isProcessRunning`))
    (`KismetSystemLibrary.PrintString` (`KismetStringLibrary.Conv_BoolToString` _returnvalue) true true (struct :`G` 0.66 :`B` 1.0 :`A` 1.0) 10.0)))

(event `Key|Three`
  (params (Key :type "Key Structure"))
  (:`Pressed`
    (`self.closeProcess` "AirRaidShelter.exe")))

(fn `UserConstructionScript`)