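; Procedural mesh Blueprint that builds a single colored polygon mesh from its Vertices array at BeginPlay.
; CreatePloy divides each vertex by 100, scales the mesh component up 100 times to compensate, and gets triangle indices from GetTriangles.
; It then applies a dynamic material instance tinted by the Color variable.
; An unconnected construction-script branch would instead fill the vertices from spline points.
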(event `self.ReceiveBeginPlay`
  (`self.CreatePloy`))

(fn `CreatePloy`
  (bind _vertices (`self.Vertices`))
  (bind _vertices_2 (`self.Vertices`))
  (for (_array_element _array_index) _vertices
    (`KismetArrayLibrary.Array_Set` _vertices _array_index (/ _array_element 100.0)))
  (`SceneComponent.SetRelativeScale3D` (`self.ProceduralMesh`) (100.0 100.0 100.0))
  (`ProceduralMeshComponent.CreateMeshSection_LinearColor` :`self` (`self.ProceduralMesh`) :`Vertices` _vertices_2 :`Triangles` (`self.GetTriangles` _vertices_2))
  (bind _returnvalue (`KismetMaterialLibrary.CreateDynamicMaterialInstance` "/Visualization/Blueprint/ProceduralMesh/ProceduralMesh_Mat.ProceduralMesh_Mat"))
  (`MaterialInstanceDynamic.SetVectorParameterValue` _returnvalue "color" (`self.Color`))
  (`PrimitiveComponent.SetMaterial` (`self.ProceduralMesh`) 0 _returnvalue))

(fn `UserConstructionScript`)