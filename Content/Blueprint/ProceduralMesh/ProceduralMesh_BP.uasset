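; Procedural mesh Blueprint that draws an outlined, colored polygon from its Vertices array on BeginPlay.
; CreateLine builds a closed linear spline from the points and adds a spline mesh component per segment.
; CreatePloy then divides Vertices in place by 100, scales the mesh up to compensate, triangulates through GetTriangles and applies a dynamic material with Color.
; The construction script's spline-to-mesh logic is disconnected.
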(event `self.ReceiveBeginPlay`
  (`self.CreateLine`)
  (`self.CreatePloy`))

(fn `CreateLine`
  (bind _spline (`self.Spline`))
  (bind _spline_2 (`self.Spline`))
  (bind _spline_3 (`self.Spline`))
  (`SplineComponent.ClearSplinePoints` _spline_2 true)
  (`SplineComponent.SetClosedLoop` _spline_2 true true)
  (for (_array_element _array_index) (`self.Vertices`)
    (`SplineComponent.AddSplinePointAtIndex` _spline _array_element _array_index "Local" true)
    (`SplineComponent.SetSplinePointType` _spline _array_index "Linear" true))
  (for _index (range (`SplineComponent.GetNumberOfSplinePoints` _spline_3))
    (bind _returnvalue (`AddComponent|NODE_AddSplineMeshComponent-0` :`bManualAttachment` true))
    (bind (_location _tangent) (`SplineComponent.GetLocationAndTangentAtSplinePoint` _spline_3 _index "Local"))
    (bind (_location_2 _tangent_2) (`SplineComponent.GetLocationAndTangentAtSplinePoint` _spline_3 (+ _index 1) "Local"))
    (`SplineMeshComponent.SetStartAndEnd` _returnvalue _location _tangent _location_2 _tangent_2 true)))

(fn `CreatePloy`
  (bind _vertices (`self.Vertices`))
  (bind _vertices_2 (`self.Vertices`))
  (for (_array_element _array_index) _vertices
    (`KismetArrayLibrary.Array_Set` _vertices _array_index (/ _array_element 100.0)))
  (`SceneComponent.SetRelativeScale3D` (`self.ProceduralMesh`) (100.0 100.0 100.0))
  (`ProceduralMeshComponent.CreateMeshSection_LinearColor` :`self` (`self.ProceduralMesh`) :`Vertices` _vertices_2 :`Triangles` (`self.GetTriangles` _vertices_2))
  (bind _returnvalue (`KismetMaterialLibrary.CreateDynamicMaterialInstance` "/Visualization/Blueprint/ProceduralMesh/ProceduralMesh_Mat.ProceduralMesh_Mat"))
  (`MaterialInstanceDynamic.SetVectorParameterValue` _returnvalue "color" (`self.Color`))
  (`PrimitiveComponent.SetMaterial` (`self.ProceduralMesh`) 0 _returnvalue))

(fn `UserConstructionScript`)