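; Mask actor that publishes a box or sphere volume to the Mask_MPC material parameter collection for materials to read.
; A Box switch shows the matching shape component, hides the other, and selects which one supplies the data.
; The Mask function writes world location, scaled bounds (full size for box, radius for sphere) and a shape flag.
; It runs on construction, BeginPlay and every Tick, keeping the parameters synced with the actor.
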(event `self.ReceiveBeginPlay`
  (`self.Mask` :!label _label))

(event `self.ReceiveTick`
  (params (DeltaSeconds :type "Float (single-precision)"))
  (goto _label))

(fn `Mask`
  (bind _sphere (`self.Sphere`))
  (bind _sphere_2 (`self.Sphere`))
  (bind _box (`self.Box`))
  (bind _box_2 (`self.Box`))
  (if (`self.bBox`)
    (`SceneComponent.SetHiddenInGame` _sphere true false)
    (`SceneComponent.SetHiddenInGame` _box_2 false false)
    (`SceneComponent.SetVisibility` _sphere false false)
    (`SceneComponent.SetVisibility` _box_2 true false)
    (`KismetMaterialLibrary.SetVectorParameterValue` "/Visualization/Blueprint/Mask/Mask_MPC.Mask_MPC" "Location" (`KismetMathLibrary.Conv_VectorToLinearColor` (`SceneComponent.K2_GetComponentLocation` _box)))
    (`KismetMaterialLibrary.SetVectorParameterValue` "/Visualization/Blueprint/Mask/Mask_MPC.Mask_MPC" "Bound" (`KismetMathLibrary.Conv_VectorToLinearColor` (* (* (`BoxComponent.BoxExtent` _box) (`SceneComponent.K2_GetComponentScale` _box)) 2.0)))
    (`KismetMaterialLibrary.SetScalarParameterValue` "/Visualization/Blueprint/Mask/Mask_MPC.Mask_MPC" "bBox" 1.0)
    (else
      (`SceneComponent.SetHiddenInGame` _sphere false false)
      (`SceneComponent.SetHiddenInGame` _box_2 true false)
      (`SceneComponent.SetVisibility` _sphere true false)
      (`SceneComponent.SetVisibility` _box_2 false false)
      (`KismetMaterialLibrary.SetVectorParameterValue` "/Visualization/Blueprint/Mask/Mask_MPC.Mask_MPC" "Location" (`KismetMathLibrary.Conv_VectorToLinearColor` (`SceneComponent.K2_GetComponentLocation` _sphere_2)))
      (`KismetMaterialLibrary.SetVectorParameterValue` "/Visualization/Blueprint/Mask/Mask_MPC.Mask_MPC" "Bound" (`KismetMathLibrary.Conv_VectorToLinearColor` (* (`SceneComponent.K2_GetComponentScale` _sphere_2) (`SphereComponent.SphereRadius` _sphere_2))))
      (`KismetMaterialLibrary.SetScalarParameterValue` "/Visualization/Blueprint/Mask/Mask_MPC.Mask_MPC" "bBox"))))

(fn `UserConstructionScript`
  (`self.Mask`))