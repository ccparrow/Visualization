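; MovieRender_BP is a Blueprint that renders a Level Sequence at runtime through Movie Render Queue shortly after play begins.
; It allocates a queue job from a preset config, setting a timestamped project output folder, resolution, sequence and map.
; An in-process executor renders it in the current level with a screen overlay.
; The job is deleted when rendering finishes, and ending play cancels any active executor's jobs.
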(event `self.ReceiveBeginPlay`
  (bind (_year _month _day _hour _minute) (`KismetMathLibrary.BreakDateTime` (`KismetMathLibrary.Now`)))
  (`KismetSystemLibrary.Delay` 1.0)
  (bind _returnvalue (`MoviePipelineQueue.AllocateNewJob` (`MoviePipelineQueueEngineSubsystem.GetQueue` (subsystem `MoviePipelineQueueEngineSubsystem`)) "/Script/MovieRenderPipelineCore.MoviePipelineExecutorJob"))
  (set `self.MovieJob` _returnvalue)
  (`MoviePipelineConfigBase.CopyFrom` (`MoviePipelineExecutorJob.GetConfiguration` (`self.MovieJob`)) (`self.MovieConfig`))
  (bind _returnvalue_2 (`MoviePipelineConfigBase.FindOrAddSettingByClass` (`MoviePipelineExecutorJob.GetConfiguration` (`self.MovieJob`)) "/Script/MovieRenderPipelineCore.MoviePipelineOutputSetting" false))
  (set `MoviePipelineOutputSetting.OutputDirectory` (make `DirectoryPath` (`KismetStringLibrary.Concat_StrStr` (`KismetSystemLibrary.GetProjectDirectory`) (`self.RenderPath`) (`KismetStringLibrary.Concat_StrStr` (`KismetStringLibrary.Conv_IntToString` _month) (`KismetStringLibrary.Conv_IntToString` _day) (`KismetStringLibrary.Conv_IntToString` _hour) (`KismetStringLibrary.Conv_IntToString` _minute) "/"))) _returnvalue_2)
  (set `MoviePipelineOutputSetting.OutputResolution` (`self.Resolution`) _returnvalue_2)
  (set `MoviePipelineExecutorJob.Sequence` (`KismetSystemLibrary.MakeSoftObjectPath` (`KismetSystemLibrary.Conv_SoftObjectReferenceToString` (`self.SequenceSoft`))) (`self.MovieJob`))
  (set `MoviePipelineExecutorJob.Map` (`KismetSystemLibrary.MakeSoftObjectPath` (`KismetSystemLibrary.Conv_SoftObjectReferenceToString` (`self.MapSoft`))) (`self.MovieJob`))
  (bind _returnvalue_3 (`|GenericCreateObject` (`self.MovieConfig`) "/Script/MovieRenderPipelineCore.MoviePipelineInProcessExecutor"))
  (add `MoviePipelineExecutorBase.OnExecutorFinishedDelegate` _returnvalue_3 (delegate `CustomEvent_0`))
  (set `MoviePipelineInProcessExecutor.bUseCurrentLevel` true _returnvalue_3)
  (set `MoviePipelineExecutorBase.DebugWidgetClass` "/MovieRenderPipeline/Blueprints/UI_MovieRenderPipelineScreenOverlay.UI_MovieRenderPipelineScreenOverlay_C" _returnvalue_3)
  (`MoviePipelineQueueEngineSubsystem.RenderQueueWithExecutorInstance` (subsystem `MoviePipelineQueueEngineSubsystem`) _returnvalue_3))

(event `CustomEvent_0`
  (params (PipelineExecutor :type "MoviePipelineExecutorBase Object Reference") (bSuccess :type Boolean))
  (`MoviePipelineQueue.DeleteJob` (`MoviePipelineQueueEngineSubsystem.GetQueue` (subsystem `MoviePipelineQueueEngineSubsystem`)) (`self.MovieJob`)))

(event `self.ReceiveEndPlay`
  (params (EndPlayReason :type "EEndPlayReason Enum" :default "Destroyed"))
  (bind _returnvalue (`MoviePipelineQueueEngineSubsystem.GetActiveExecutor` (subsystem `MoviePipelineQueueEngineSubsystem`)))
  (`/Engine/EditorBlueprintResources/StandardMacros.IsValid` (`self.MovieJob`)
    (:`Is Valid`
      (if (`KismetSystemLibrary.IsValid` _returnvalue)
        (`MoviePipelineExecutorBase.CancelAllJobs` _returnvalue)))))

(fn `UserConstructionScript`)