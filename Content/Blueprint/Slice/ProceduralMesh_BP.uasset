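; Blueprint actor that stands in for a referenced static mesh so it can be sliced at runtime.
; BeginPlay hides the static mesh and copies it into a ProceduralMesh; destruction makes the original visible again.
; Slice_Event cuts along a given plane with an optional flipped normal, creating a capped other half and applying a replacement material to it.
; CopyMesh restores the procedural mesh from the source once a slice has occurred.
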(event `self.ReceiveBeginPlay`
  (bind _staticmeshcomp_ref (`self.StaticMeshComp_Ref`))
  (`/Engine/EditorBlueprintResources/StandardMacros.IsValid` _staticmeshcomp_ref
    (:`Is Valid`
      (`SceneComponent.SetVisibility` _staticmeshcomp_ref false false)
      (`KismetProceduralMeshLibrary.CopyProceduralMeshFromStaticMeshComponent` _staticmeshcomp_ref 0 (`self.ProceduralMesh`)))))

(event `Slice_Event`
  (params (PlanePosition :type "Vector Structure") (PlaneNormal :type "Vector Structure" :default (0.0 1.0 0.0)))
  (bind _outotherhalfprocmesh (`KismetProceduralMeshLibrary.SliceProceduralMesh` (`self.ProceduralMesh`) PlanePosition (`KismetMathLibrary.SelectVector` (* PlaneNormal -1) PlaneNormal (`self.bFlipNormal`)) true "CreateNewSectionForCap" (`PrimitiveComponent.GetMaterial` (`self.StaticMeshComp_Ref`) 0)))
  (for (_ _array_index) (`MeshComponent.GetMaterials` (`self.StaticMeshComp_Ref`))
    (`PrimitiveComponent.SetMaterial` _outotherhalfprocmesh _array_index (`self.ProceduralMat_Ref`)))
  (set `self.bSlice` true))

(event `self.ReceiveDestroyed`
  (`/Engine/EditorBlueprintResources/StandardMacros.IsValid` (`self.StaticMeshComp_Ref`)
    (:`Is Valid`
      (`SceneComponent.SetVisibility` (`self.StaticMeshComp_Ref`) true false))))

(fn `CopyMesh`
  (if (`self.bSlice`)
    (`KismetProceduralMeshLibrary.CopyProceduralMeshFromStaticMeshComponent` (`self.StaticMeshComp_Ref`) 0 (`self.ProceduralMesh`)))
  (return))

(fn `UserConstructionScript`)