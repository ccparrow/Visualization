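; Movable slicing-plane actor that cuts overlapped static meshes through procedural mesh proxies, tinted by a configurable color.
; Box or Plane overlaps spawn a ProceduralMesh_BP per static mesh component, tracked in a map and destroyed on overlap end.
; Keys 1 and 2 move it along its right axis via timelines, slicing every update with AlwaysSlice, otherwise on release.
; SliceMesh respawns already-sliced proxies from their source component before cutting at the actor's plane.
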(event `self.ReceiveBeginPlay`
  (`self.EnableInput` (`GameplayStatics.GetPlayerController` 0)))

(event `Key|One`
  (params (Key :type "Key Structure"))
  (:`Pressed`
    (`Timeline|Timeline_0` :!label _label
      (:`Update`
        (`self.K2_AddActorWorldOffset` (* (`self.GetActorRightVector`) (`self.MoveSpeed`)))
        (if (`self.bAlwaysSlice`) :!label _label_2
          (`self.SliceMesh`)))))
  (:`Released`
    (if (`self.bAlwaysSlice`)
      (goto _label :!via `Stop`)
      (else
        (`self.SliceMesh`)
        (goto _label :!via `Stop`)))))

(event `Key|Two`
  (params (Key :type "Key Structure"))
  (:`Pressed`
    (`Timeline|Timeline_1` :!label _label_3
      (:`Update`
        (`self.K2_AddActorWorldOffset` (* (* (`self.GetActorRightVector`) -1) (`self.MoveSpeed`)))
        (goto _label_2))))
  (:`Released`
    (if (`self.bAlwaysSlice`)
      (goto _label_3 :!via `Stop`)
      (else
        (`self.SliceMesh`)
        (goto _label_3 :!via `Stop`)))))

(event `self.Box.OnComponentBeginOverlap`
  (params (OverlappedComponent :type "PrimitiveComponent Object Reference") (OtherActor :type "Actor Object Reference") (OtherComp :type "PrimitiveComponent Object Reference") (OtherBodyIndex :type Integer) (bFromSweep :type Boolean) (SweepResult :type "HitResult Structure (by ref)"))
  (`self.AddProcedural` OtherComp :!label _label_4)
  (`V_Library.PrintTo` "Visualization"))

(event `self.Plane.OnComponentBeginOverlap`
  (params (OverlappedComponent :type "PrimitiveComponent Object Reference") (OtherActor :type "Actor Object Reference") (OtherComp :type "PrimitiveComponent Object Reference") (OtherBodyIndex :type Integer) (bFromSweep :type Boolean) (SweepResult :type "HitResult Structure (by ref)"))
  (goto _label_4))

(event `self.Box.OnComponentEndOverlap`
  (params (OverlappedComponent :type "PrimitiveComponent Object Reference") (OtherActor :type "Actor Object Reference") (OtherComp :type "PrimitiveComponent Object Reference") (OtherBodyIndex :type Integer))
  (`self.RemoveProcedural` OtherComp :!label _label_5)
  (`V_Library.PrintTo` "11111Visualization"))

(event `self.Plane.OnComponentEndOverlap`
  (params (OverlappedComponent :type "PrimitiveComponent Object Reference") (OtherActor :type "Actor Object Reference") (OtherComp :type "PrimitiveComponent Object Reference") (OtherBodyIndex :type Integer))
  (goto _label_5))

(fn `AddProcedural`
  (params (Comp :type "PrimitiveComponent Object Reference"))
  (returns (Procedural :type "/Visualization/Blueprint/Slice/ProceduralMesh_BP Object Reference"))
  (bind _asstatic_mesh_component (cast `StaticMeshComponent` Comp))
  (bind _returnvalue (`|SpawnActorFromClass` "/Visualization/Blueprint/Slice/ProceduralMesh_BP.ProceduralMesh_BP_C" (`SceneComponent.K2_GetComponentToWorld` _asstatic_mesh_component) "AlwaysSpawn" "OverrideRootScale" null _asstatic_mesh_component false null))
  (`BlueprintMapLibrary.Map_Add` (`self.ProceduralArray`) _returnvalue _asstatic_mesh_component)
  (return _returnvalue))

(fn `ReloadProcedural`
  (params (Procedural :type "/Visualization/Blueprint/Slice/ProceduralMesh_BP Object Reference") (Index :type Integer))
  (returns (NewProcedural :type "/Visualization/Blueprint/Slice/ProceduralMesh_BP Object Reference"))
  (locals (LStaticComp :type "StaticMeshComponent Object Reference"))
  (bind _values (`BlueprintMapLibrary.Map_Values` (`self.ProceduralArray`)))
  (set `local.LStaticComp` (`|GetArrayItem` _values Index))
  (`self.K2_DestroyActor` Procedural)
  (`BlueprintMapLibrary.Map_Remove` (`self.ProceduralArray`) Procedural)
  (bind _procedural (`self.AddProcedural` (`local.LStaticComp`)))
  (return _procedural))

(fn `RemoveProcedural`
  (params (Comp :type "PrimitiveComponent Object Reference"))
  (bind _proceduralarray (`self.ProceduralArray`))
  (bind _asstatic_mesh_component (cast `StaticMeshComponent` Comp))
  (bind _values (`BlueprintMapLibrary.Map_Values` _proceduralarray))
  (if (`KismetArrayLibrary.Array_Contains` _values _asstatic_mesh_component)
    (bind _keys (`BlueprintMapLibrary.Map_Keys` _proceduralarray))
    (bind _output (`|GetArrayItem` _keys (`KismetArrayLibrary.Array_Find` _values _asstatic_mesh_component)))
    (`self.K2_DestroyActor` _output)
    (`BlueprintMapLibrary.Map_Remove` (`self.ProceduralArray`) _output)))

(fn `SliceMesh`
  (bind _returnvalue (`self.K2_GetActorLocation`))
  (bind _returnvalue_2 (`self.GetActorRightVector`))
  (bind _keys (`BlueprintMapLibrary.Map_Keys` (`self.ProceduralArray`)))
  (for (_array_element _array_index) _keys
    (if (`/Visualization/Blueprint/Slice/ProceduralMesh_BP.bSlice` _array_element)
      (bind _newprocedural (`self.ReloadProcedural` _array_element _array_index))
      (`/Visualization/Blueprint/Slice/ProceduralMesh_BP.Slice_Event` _newprocedural _returnvalue _returnvalue_2)
      (else
        (`/Visualization/Blueprint/Slice/ProceduralMesh_BP.Slice_Event` _array_element _returnvalue _returnvalue_2)))))

(fn `UserConstructionScript`
  (bind _color (`self.Color`))
  (bind _returnvalue (`KismetMaterialLibrary.CreateDynamicMaterialInstance` "/Visualization/Blueprint/Slice/Slice_Mat.Slice_Mat"))
  (`PrimitiveComponent.SetMaterial` (`self.Plane`) 0 _returnvalue)
  (`PrimitiveComponent.SetMaterial` (`self.Plane1`) 0 _returnvalue)
  (`MaterialInstanceDynamic.SetVectorParameterValue` _returnvalue "EmissiveColor" _color)
  (`MaterialInstanceDynamic.SetScalarParameterValue` _returnvalue "OpacityIntensity" (`.A` (break `LinearColor` _color))))