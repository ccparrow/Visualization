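; Test Blueprint that exercises Aliyun OSS cloud storage calls when play begins.
; BeginPlay creates a bucket and prints the result, then after a short delay lists the stored objects and prints each name.
; An unconnected GetObject branch would download each listed object to a hardcoded F: drive path, but it never runs.
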(event `self.ReceiveBeginPlay`
  (bind _returnvalue (`self.CreateBucket` ""))
  (`V_Library.PrintTo` (`KismetStringLibrary.Conv_BoolToString` _returnvalue))
  (`KismetSystemLibrary.Delay` 2.0)
  (bind _namearray (`self.ListObject`))
  (for _array_element _namearray
    (`KismetSystemLibrary.PrintString` _array_element)))

(fn `UserConstructionScript`)