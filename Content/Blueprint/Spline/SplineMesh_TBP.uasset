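; Construction-script Blueprint that lays a static mesh along a spline, either its own or one from a picked SplinePick.
; AddMesh rounds spline length over mesh bounds Max X to get evenly stretched spline mesh segments, applying X scale and an offset in spline space.
; Flipping mirrors via negative Y component scale, with compensated positions and tangents.
; When Material is set, each segment gets a dynamic material instance stored in MaterialArray.
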(fn `AddMesh`
  (params (Spline :type "SplineComponent Object Reference") (StaticMesh :type "StaticMesh Object Reference") (FlipMesh :type Boolean) (ScaleX :type "Float (double-precision)") (Offset :type "Vector Structure"))
  (returns (MeshArray :type "Array of SplineMeshComponent Object Reference"))
  (locals (LNumber :type Integer) (LLength :type "Float (double-precision)" :default 0.0) (LFlipMesh :type Boolean :default false) (LOffset :type "Vector Structure" :default (0.0 0.0 0.0)) (LSpline :type "SplineComponent Object Reference") (LStaticMesh :type "StaticMesh Object Reference") (LMeshArrayOut :type "Array of SplineMeshComponent Object Reference") (LainLine :type Boolean) (_ScaleX :type "Float (double-precision)"))
  (bind _lspline (`local.LSpline`))
  (bind __scalex (`local._ScaleX`))
  (bind _returnvalue (`StaticMesh.GetBoundingBox` (`local.LStaticMesh`)))
  (bind (_remainder _returnvalue_2) (`KismetMathLibrary.FMod` (`SplineComponent.GetSplineLength` (`local.LSpline`)) (.x (`.Max` (break `Box` _returnvalue)))))
  (bind _returnvalue_3 (`KismetMathLibrary.MakeVector` 1.0 (`KismetMathLibrary.SelectFloat` -1.0 1.0 (`local.LFlipMesh`)) 1.0))
  (set `local.LSpline` Spline)
  (`/Engine/EditorBlueprintResources/StandardMacros.IsValid` StaticMesh
    (:`Is Valid`
      (set `local.LStaticMesh` StaticMesh)
      (set `local.LFlipMesh` FlipMesh)
      (set `local._ScaleX` ScaleX)
      (set `local.LOffset` Offset)
      ;[1 1 1] 模型段数
      (set `local.LNumber` (select `bool` (>= _remainder (* (.x (`.Max` (break `Box` _returnvalue))) 0.5)) :`false` (`KismetMathLibrary.Max` _returnvalue_2 1) :`true` (+ _returnvalue_2 1)))
      ;[1 1 1] 单位长度
      (set `local.LLength` (/ (`SplineComponent.GetSplineLength` (`local.LSpline`)) (`KismetMathLibrary.Conv_IntToDouble` (`local.LNumber`))))
      (`KismetArrayLibrary.Array_Clear` (`local.LMeshArrayOut`))
      (for _index (range (`local.LNumber`))
        (bind _returnvalue_4 (`AddComponent|NODE_AddSplineMeshComponent-3` :`RelativeTransform` (`KismetMathLibrary.MakeTransform` (0.0 0.0 0.0) (struct) (`KismetMathLibrary.MakeVector` 1.0 (`KismetMathLibrary.SelectFloat` -1.0 1.0 (`local.LFlipMesh`)) 1.0))))
        (`KismetArrayLibrary.Array_Add` (`local.LMeshArrayOut`) _returnvalue_4)
        (`StaticMeshComponent.SetStaticMesh` _returnvalue_4 (`local.LStaticMesh`))
        (`SplineMeshComponent.SetStartScale` _returnvalue_4 (`KismetMathLibrary.MakeVector2D` __scalex 1.0) true)
        (`SplineMeshComponent.SetEndScale` _returnvalue_4 (`KismetMathLibrary.MakeVector2D` __scalex 1.0) true)
        (bind _returnvalue_5 (* _index (`local.LLength`)))
        (bind _returnvalue_6 (+ _returnvalue_5 (`local.LLength`)))
        (`SplineMeshComponent.SetStartAndEnd` _returnvalue_4 (* (+ (`SplineComponent.GetLocationAtDistanceAlongSpline` _lspline _returnvalue_5 "Local") (`KismetMathLibrary.TransformDirection` (`SplineComponent.GetTransformAtDistanceAlongSpline` _lspline _returnvalue_5 "Local" true) (`local.LOffset`))) _returnvalue_3) (* (* (`SplineComponent.GetDirectionAtDistanceAlongSpline` _lspline _returnvalue_5 "Local") (`local.LLength`)) _returnvalue_3) (* _returnvalue_3 (+ (`SplineComponent.GetLocationAtDistanceAlongSpline` _lspline _returnvalue_6 "Local") (`KismetMathLibrary.TransformDirection` (`SplineComponent.GetTransformAtDistanceAlongSpline` _lspline _returnvalue_6 "Local" true) (`local.LOffset`)))) (* _returnvalue_3 (* (`SplineComponent.GetDirectionAtDistanceAlongSpline` _lspline _returnvalue_6 "Local") (`local.LLength`))) true))
      (return (`local.LMeshArrayOut`)))))

(fn `MaterialInstance`
  (params (Array :type "Array of SplineMeshComponent Object Reference"))
  (for _array_element Array
    (bind _returnvalue (`PrimitiveComponent.CreateDynamicMaterialInstance` _array_element 0 null "None"))
    (`KismetArrayLibrary.Array_Add` (`self.MaterialArray`) _returnvalue)))

(fn `UserConstructionScript`
  (locals (_Spline :type "SplineComponent Object Reference"))
  (bind _splinepick (`self.SplinePick`))
  ;[1 1 1] 刷新
  (`/Engine/EditorBlueprintResources/StandardMacros.IsValid` _splinepick
    (:`Is Valid`
      (set `local._Spline` (`/Game/Blueprint/Spline/SplineMesh_TBP.Spline` _splinepick)))
    (:`Is Not Valid`
      (set `local._Spline` (`self.Spline`))))
  (if (`self.Refresh`)
    (set `self.Refresh` false))
  (`KismetArrayLibrary.Array_Clear` (`self.MaterialArray`))
  ;[1 1 1] 添加模型
  (bind _mesharray (`self.AddMesh` (`local._Spline`) (`self.StaticMesh`) (`self.bFlipMesh`) (`self.ScaleX`) (`self.Offset`)))
  (if (`self.bMaterial`)
    (`self.MaterialInstance` _mesharray)))