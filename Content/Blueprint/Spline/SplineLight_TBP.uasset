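; Spline light Blueprint that places a row of spot lights along a spline and shows them only at night.
; The construction script uses an assigned actor's spline or its own, adding lights at each spline point or at a set spacing, optionally evened out over the length.
; It also applies an initial visibility setting.
; At BeginPlay it binds to the VGIS night event, which toggles root visibility and propagates to children.
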(event `self.ReceiveBeginPlay`
  (add `/Visualization/GamePlay/VGIS.Night_ED` (subsystem `/Visualization/GamePlay/VGIS`) (delegate `CustomEvent_0`)))

(event `CustomEvent_0`
  (params (bNight :type Boolean))
  (bind _defaultsceneroot (`self.DefaultSceneRoot`))
  (`SceneComponent.SetVisibility` _defaultsceneroot bNight true)
  (`SceneComponent.SetHiddenInGame` _defaultsceneroot (not bNight) true))

(fn `UserConstructionScript`
  (bind _splineactor (`self.SplineActor`))
  (bind _splineref (`self.SplineRef`))
  (bind _returnvalue (`SplineComponent.GetSplineLength` (`self.SplineRef`)))
  (bind _returnvalue_2 (`self.GetComponentByClass` _splineactor "/Script/Engine.SplineComponent"))
  (bind _returnvalue_3 (`KismetMathLibrary.FFloor` (/ _returnvalue (`self.Distance`))))
  (`|ExecutionSequence`
    (:`then_0`
      (`/Engine/EditorBlueprintResources/StandardMacros.IsValid` _splineactor
        (:`Is Valid`
          (`/Engine/EditorBlueprintResources/StandardMacros.IsValid` _returnvalue_2
            (:`Is Valid`
              (set `self.SplineRef` _returnvalue_2))))
        (:`Is Not Valid`
          (set `self.SplineRef` (`self.Spline`))))
      (if (`self.UseSplinePoint?`)
        (for _index (range (`SplineComponent.GetNumberOfSplinePoints` _splineref))
          (`AddComponent|NODE_AddSpotLightComponent-0` :`RelativeTransform` (`KismetMathLibrary.MakeTransform` (`KismetMathLibrary.SelectVector` (`SplineComponent.GetLocationAtSplinePoint` _splineref _index "Local") (`SplineComponent.GetLocationAtDistanceAlongSpline` (`self.SplineRef`) (* (`KismetMathLibrary.Conv_IntToDouble` (stale _index_2)) (`self.Distance`)) "Local") (`self.UseSplinePoint?`)) (struct :`Pitch` -90.0)) :!label _label))
        (else
          (if (`self.AverageDistance?`)
            (set `self.Distance` (/ _returnvalue (`KismetMathLibrary.Conv_IntToDouble` _returnvalue_3))))
          (for _index_2 (range (+ _returnvalue_3 1))
            (goto _label)))))
    (:`then_1`
      (`SceneComponent.SetVisibility` (`self.DefaultSceneRoot`) (`self.bVisibility`) true))))