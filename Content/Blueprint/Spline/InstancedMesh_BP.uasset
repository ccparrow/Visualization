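; Spline-based scattering Blueprint that places instances of a chosen static mesh along a spline in its construction script.
; Instances sit either on each spline point or at a set distance interval, which can be adjusted to divide the spline length evenly.
; Both modes share one AddInstance step that orients meshes to the spline tangent, with optional random yaw, and randomly varies the scale around a base scalar.
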(fn `UserConstructionScript`
  (bind _spline (`self.Spline`))
  (bind _usesplinepoint_ (`self.UseSplinePoint?`))
  (bind _spline_2 (`self.Spline`))
  (bind _returnvalue (`SplineComponent.GetSplineLength` (`self.Spline`)))
  (bind _returnvalue_2 (`KismetMathLibrary.FFloor` (/ _returnvalue (`self.Distance`))))
  (`StaticMeshComponent.SetStaticMesh` (`self.InstancedMesh`) (`self.StaticMesh`))
  (if (`self.UseSplinePoint?`)
    (for _index (range (`SplineComponent.GetNumberOfSplinePoints` _spline_2))
      (bind _returnvalue_3 (* (`KismetMathLibrary.Conv_IntToDouble` (stale _index_2)) (`self.Distance`)))
      (`InstancedStaticMeshComponent.AddInstance` (`self.InstancedMesh`) (`KismetMathLibrary.MakeTransform` (`KismetMathLibrary.SelectVector` (`SplineComponent.GetLocationAtSplinePoint` _spline_2 _index "Local") (`SplineComponent.GetLocationAtDistanceAlongSpline` _spline _returnvalue_3 "Local") _usesplinepoint_) (`KismetMathLibrary.MakeRotator` (.roll (`KismetMathLibrary.Conv_VectorToRotator` (`KismetMathLibrary.SelectVector` (`SplineComponent.GetTangentAtSplinePoint` _spline _index "Local") (`SplineComponent.GetTangentAtDistanceAlongSpline` _spline _returnvalue_3 "Local") _usesplinepoint_))) (.pitch (`KismetMathLibrary.Conv_VectorToRotator` (`KismetMathLibrary.SelectVector` (`SplineComponent.GetTangentAtSplinePoint` _spline _index "Local") (`SplineComponent.GetTangentAtDistanceAlongSpline` _spline _returnvalue_3 "Local") _usesplinepoint_))) (`KismetMathLibrary.SelectFloat` (`KismetMathLibrary.RandomFloatInRange` 0.0 360.0) (.yaw (`KismetMathLibrary.Conv_VectorToRotator` (`KismetMathLibrary.SelectVector` (`SplineComponent.GetTangentAtSplinePoint` _spline _index "Local") (`SplineComponent.GetTangentAtDistanceAlongSpline` _spline _returnvalue_3 "Local") _usesplinepoint_))) (`self.bRandomRotationZ`))) (* (`self.MeshScalar`) (`KismetMathLibrary.RandomFloatInRange` 0.7 1.2))) :!label _label))
    (else
      (if (`self.AverageDistance?`)
        (set `self.Distance` (/ _returnvalue (`KismetMathLibrary.Conv_IntToDouble` _returnvalue_2))))
      (for _index_2 (range (+ _returnvalue_2 1))
        (goto _label)))))