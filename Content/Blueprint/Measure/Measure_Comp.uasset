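; Measurement component that lets the player drag out a distance between two points in the world.
; MeasureStart traces for an object under the click, stores the hit as the start point, spawns a Measure_BP marker there and starts a looping timer.
; Each timer tick re-traces and updates the marker's end point and rounded centimeter label.
; MeasureEnd pauses the timer, leaving the spawned marker in place.
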(fn `_MeasureDrag`
  (bind (_outhit _returnvalue) (`/Visualization/GamePlay/Visual_BPLibrary.ClickForObject` (`self._ObjectTypeArray`) (`|MakeArray` null :!type "Actor Object Reference")))
  (if _returnvalue
    (set `self._EndPoint` (`.Location` (`GameplayStatics.BreakHitResult` _outhit)))
    (set `self._Distance` (`KismetMathLibrary.Vector_Distance` (`self._StartPoint`) (`self._EndPoint`)))
    (`/Visualization/Blueprint/Measure/Measure_BP.SetEndPoint` (`self._Measure_Ref`) (`self._EndPoint`) (`KismetTextLibrary.Conv_StringToText` (`KismetStringLibrary.Concat_StrStr` (`KismetStringLibrary.Conv_IntToString` (`KismetMathLibrary.Round` (`self._Distance`))) " cm")))))

(fn `MeasureEnd`
  (`KismetSystemLibrary.K2_PauseTimer` null "_MeasureDrag"))

(fn `MeasureStart`
  (bind (_outhit _returnvalue) (`/Visualization/GamePlay/Visual_BPLibrary.ClickForObject` (`self._ObjectTypeArray`) (`|MakeArray` null :!type "Actor Object Reference")))
  (if _returnvalue
    (bind _output_get (set `self._StartPoint` (`.Location` (`GameplayStatics.BreakHitResult` _outhit))))
    (bind _returnvalue_2 (`|SpawnActorFromClass` "/Visualization/Blueprint/Measure/Measure_BP.Measure_BP_C" (`KismetMathLibrary.MakeTransform` _output_get (struct) (5.0 5.0 5.0)) "AlwaysSpawn" "OverrideRootScale" null null))
    (set `self._Measure_Ref` _returnvalue_2)
    (`KismetSystemLibrary.K2_SetTimer` null "_MeasureDrag" 0.02 true)))