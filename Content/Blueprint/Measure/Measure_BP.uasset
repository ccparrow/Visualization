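; Measurement marker actor that draws a labeled line between its start point and an end location.
; SetEndPoint, run from the Construction Script, aims the root at the end location, moves the end mesh and cable end there, and centers the text label along the cable.
; Visiable toggles in-game visibility of both meshes and the label, propagating to children, and BeginPlay hides them initially.
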(event `self.ReceiveBeginPlay`
  (`self.Visiable` false))

(fn `SetEndPoint`
  (params (EndLocation :type "Vector Structure") (Text :type Text))
  (`SceneComponent.K2_SetWorldRotation` (`self.Root`) (`KismetMathLibrary.FindLookAtRotation` (`self.K2_GetActorLocation`) EndLocation) false false) ; 旋转垂直于横线
  (`SceneComponent.K2_SetWorldLocation` (`self.EndMesh`) EndLocation false false) ; 终点位置
  (`TextRenderComponent.K2_SetText` (`self.TextRender`) Text) ; 文字内容
  (bind _output_get (set `CableComponent.EndLocation` (`SceneComponent.RelativeLocation` (`self.EndMesh`)) (`self.Cable`)))
  (`SceneComponent.K2_SetRelativeLocation` (`self.TextRender`) (/ _output_get 2.0) false false) ; 文字位置
)

(fn `UserConstructionScript`
  (`self.SetEndPoint` (`self.EndLocation`) (`self.Text`)))

(fn `Visiable`
  (params (bvisiable :type Boolean))
  (bind _output_get (set `self.bvisiable` bvisiable))
  (`SceneComponent.SetHiddenInGame` (`self.EndMesh`) (not _output_get) true)
  (`SceneComponent.SetHiddenInGame` (`self.TextRender`) (not _output_get) true)
  (`SceneComponent.SetHiddenInGame` (`self.StartMesh`) (not _output_get) true))