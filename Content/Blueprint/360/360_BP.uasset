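; 360 panorama hotspot actor with a labeled, clickable tag widget and a sphere showing a per-instance texture set in the construction script.
; Entering saves the pawn transform, timeline-scales the sphere up from zero and focuses Visual_Pawn inside it.
; In editor it adds a close-button widget; otherwise it sends a panorama message through Visual_GameState Pixel Streaming.
; Exiting restores the saved view and reverses the sphere animation.
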(event `self.ReceiveBeginPlay`
  (bind _as360tag_wbp (cast `/Visualization/Blueprint/360/360Tag_WBP` (`WidgetComponent.GetUserWidgetObject` (`self.Widget`))))
  (set `/Visualization/Blueprint/360/360Tag_WBP.Text` (`self.Text`) _as360tag_wbp)
  (add `/Visualization/Blueprint/360/360Tag_WBP.Clicked_ED` _as360tag_wbp (`|CreateDelegate` :!event `In360_Event`))
  (`SceneComponent.SetRelativeScale3D` (`self.Sphere`) (0.0 0.0 0.0)))

(event `In360_Event`
  (bind _returnvalue (`GameplayStatics.GetPlayerPawn` 0))
  (bind _returnvalue_2 (`self.K2_GetActorRotation` _returnvalue))
  (`SceneComponent.SetVisibility` (`self.Sphere`) true false)
  (`self.PlaySphere_Event`)
  (bind _asvisual_pawn (cast `/Visualization/GamePlay/Visual_Pawn` _returnvalue))
  (set `self.RotationSave` _returnvalue_2)
  (set `self.LocationSave` (`self.K2_GetActorLocation` _returnvalue))
  (`/Visualization/GamePlay/Visual_Pawn.FocusLocation_Event` _asvisual_pawn (`SceneComponent.K2_GetComponentLocation` (`self.Sphere`)) (`KismetMathLibrary.MakeRotator` 0.0 0.0 (.yaw _returnvalue_2)) 0.0)
  (`V_Library.IsEditor`
    (:`Success`
      (bind _returnvalue_3 (`|CreateWidget` "/Visualization/Blueprint/360/360Close_WBP.360Close_WBP_C"))
      (`UserWidget.AddToViewport` _returnvalue_3 0)
      (add `/Visualization/Blueprint/360/360Close_WBP.Clicked_ED` _returnvalue_3 (`|CreateDelegate` :!event `Out360_Event`)))
    (:`Fail`
      (bind _asvisual_game_state (cast `/Visualization/GamePlay/Visual_GameState` (`GameplayStatics.GetGameState`)))
      (`/Visualization/GamePlay/Visual_GameState.SendPixelStreaming` _asvisual_game_state "" "123456" "panorama" "0"))))

(event `Out360_Event`
  (bind _asvisual_pawn (cast `/Visualization/GamePlay/Visual_Pawn` (`GameplayStatics.GetPlayerPawn` 0)))
  (`/Visualization/GamePlay/Visual_Pawn.FocusLocation_Event` _asvisual_pawn (`self.LocationSave`) (`self.RotationSave`) 0.0)
  (`self.ReverseSphere_Event`)
  (`V_Library.IsEditor`
    (:`Success`
      (`Widget.RemoveFromParent` (stale `In360_Event` _returnvalue_3)))
    (:`Fail`
      _))
  (`KismetSystemLibrary.Delay` 2.0))

(event `HiddenTag_Event`
  (params (bHidden :type Boolean))
  (`SceneComponent.SetHiddenInGame` (`self.Widget`) bHidden false))

(event `PlaySphere_Event`
  (bind (_direction _scale) (`Timeline|Timeline_0` :!via `PlayFromStart` :!label _label)
    (:`Update`
      (`SceneComponent.SetRelativeScale3D` (`self.Sphere`) (`KismetMathLibrary.Conv_DoubleToVector` _scale)))))

(event `ReverseSphere_Event`
  (goto _label :!via `ReverseFromEnd`))

(fn `UserConstructionScript`
  (bind _returnvalue (`PrimitiveComponent.CreateDynamicMaterialInstance` (`self.Sphere`) 0 null "None"))
  (`MaterialInstanceDynamic.SetTextureParameterValue` _returnvalue "texture" (`self.Texture`)))