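; Component that lets the player select objects with the mouse and drag them through a Gizmo_BP actor spawned at BeginPlay.
; GizmoStart traces under the cursor in two phases: a WorldDynamic hit readies the gizmo and switches tracing to PhysicsBody, whose hits start dragging.
; Dragging runs on a looping timer with the gizmo's UI shown until GizmoEnd; a missed trace hides the gizmo and resets the trace type.
; Setters forward local-space and snap settings, with GizmoType also writing Local.
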(event `self.ReceiveBeginPlay`
  (bind _returnvalue (`|SpawnActorFromClass` "/Visualization/Blueprint/Gizmo/Blueprint/Gizmo_BP.Gizmo_BP_C" (`KismetMathLibrary.MakeTransform` (0.0 0.0 0.0)) "AlwaysSpawn" "OverrideRootScale" null null)) ; 开始生成坐标轴
  (set `self._GizmoBPRef` _returnvalue))

(fn `_GizmoDrag`
  (`/Visualization/Blueprint/Gizmo/Blueprint/Gizmo_BP.GizmoDrag` (`self._GizmoBPRef`)) ; 拖动
)

(fn `GizmoEnd`
  (bind _ui_ref (`/Visualization/Blueprint/Gizmo/Blueprint/Gizmo_BP.UI_Ref` (`self._GizmoBPRef`)))
  (`KismetSystemLibrary.K2_PauseTimer` null "_GizmoDrag") ; 停止拖动
  (`/Engine/EditorBlueprintResources/StandardMacros.IsValid` _ui_ref
    (:`Is Valid`
      (`Widget.RemoveFromParent` _ui_ref))))

(fn `GizmoLocal`
  (params (bLocal :type Boolean :default true))
  (set `/Visualization/Blueprint/Gizmo/Blueprint/Gizmo_BP.bLocal` bLocal (`self._GizmoBPRef`)))

(fn `GizmoSnap`
  (params (bSnap :type Boolean :default true))
  (set `/Visualization/Blueprint/Gizmo/Blueprint/Gizmo_BP.bSnap` bSnap (`self._GizmoBPRef`)))

(fn `GizmoStart`
  (returns (Value :type Boolean) (Actor :type "Actor Object Reference"))
  (locals (_Value :type Boolean :default true) (_Actor :type "Actor Object Reference"))
  (bind (_worldlocation _worlddirection) (`PlayerController.DeprojectMousePositionToWorld` (`GameplayStatics.GetPlayerController` 0)))
  (bind _ui_ref (`/Visualization/Blueprint/Gizmo/Blueprint/Gizmo_BP.UI_Ref` (`self._GizmoBPRef`)))
  (bind (_outhit _returnvalue) (`KismetSystemLibrary.LineTraceSingleForObjects` _worldlocation (+ _worldlocation (* _worlddirection (`PlayerController.HitResultTraceDistance` (`GameplayStatics.GetPlayerController` 0)))) (`|MakeArray` (`self._TraceType`)) false (`|MakeArray` (`GameplayStatics.GetPlayerPawn` 0) :!type "Actor Object Reference"))) ; 射线检测物体
  (bind _output_get (set `local._Value` _returnvalue))
  (set `local._Actor` (`.HitActor` (`GameplayStatics.BreakHitResult` _outhit)))
  (if _output_get
    (`/Visualization/Blueprint/Gizmo/Blueprint/Gizmo_BP.GizmoReady` (`self._GizmoBPRef`) _outhit)
    (switch `EObjectTypeQuery` (`self._TraceType`)
      (:`ObjectTypeQuery2`
        (set `self._TraceType` "ObjectTypeQuery4") ; 坐标类型
      )
      (:`ObjectTypeQuery4`
        (`KismetSystemLibrary.K2_SetTimer` null "_GizmoDrag" 0.02 true) ; 持续执行拖动
        (`/Engine/EditorBlueprintResources/StandardMacros.IsValid` _ui_ref
          (:`Is Valid`
            (`UserWidget.AddToViewport` _ui_ref 0)))))
    (return (`local._Value`) (`local._Actor`))
    (else
      ;[1 1 1] 重置状态
      (set `self._TraceType` "ObjectTypeQuery2") ; 交互物体类型
      (`Actor.SetActorHiddenInGame` (`self._GizmoBPRef`) true)
      (return (`local._Value`) (`local._Actor`)))))

(fn `GizmoType`
  (params (bLocalType :type Boolean :default false))
  (set `/Visualization/Blueprint/Gizmo/Blueprint/Gizmo_BP.bLocal` bLocalType (`self._GizmoBPRef`)))