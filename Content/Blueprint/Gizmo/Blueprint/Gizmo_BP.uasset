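; Runtime transform gizmo actor that moves, rotates and scales a clicked actor with colored X/Y/Z handles, keeping constant screen size.
; GizmoReady attaches to the hit actor or, on a handle hit, highlights it and saves the starting transform and cursor point on a virtual plane.
; GizmoDrag uses handle tags for mode and axis, applying the cursor's plane offset with optional local space and snapping.
; The edited value feeds a Gizmo_UI widget's text.
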(event `self.ReceiveBeginPlay`
  (`self.SetActorHiddenInGame` true) ; 开始隐藏
  (bind _returnvalue (`|CreateWidget` "/Visualization/Blueprint/Gizmo/UMG/Gizmo_UI.Gizmo_UI_C"))
  (set `self.UI_Ref` _returnvalue))

(event `self.ReceiveTick`
  (params (DeltaSeconds :type "Float (single-precision)"))
  (if (not (`self.bHidden`))
    (`self.GizmoSize`) ; 保持坐标轴相对屏幕大小不变
  ))

(fn `GizmoDrag`
  (bind _returnvalue (`GameplayStatics.GetPlayerController` 0))
  (bind _returnvalue_2 (`KismetMathLibrary.MakeTransform` (`self.LocationSave`) (`self.RotationSave`) (`self.ScaleSave`)))
  (bind (_locationx _locationy) (`PlayerController.GetMousePosition` _returnvalue))
  (bind (_worldposition _worlddirection) (`GameplayStatics.DeprojectScreenToWorld` _returnvalue (`KismetMathLibrary.MakeVector2D` _locationx _locationy)))
  (bind _returnvalue_3 (`KismetStringLibrary.Conv_StringToInt` (`KismetStringLibrary.Conv_NameToString` (`|GetArrayItem` (`ActorComponent.ComponentTags` (`self.ComponentRef`)) 1))))
  (bind _returnvalue_4 (`KismetStringLibrary.Conv_StringToInt` (`KismetStringLibrary.Conv_NameToString` (`|GetArrayItem` (`ActorComponent.ComponentTags` (`self.ComponentRef`)) 1))))
  (bind _returnvalue_5 (- (`.Intersection` (`KismetMathLibrary.LinePlaneIntersection` _worldposition (+ _worldposition (* _worlddirection (`PlayerController.HitResultTraceDistance` _returnvalue))) (`self.VirtualPlaneSave`))) (`self.VirtualPositionSave`)))
  (bind _returnvalue_6 (`KismetMathLibrary.ProjectVectorOnToVector` _returnvalue_5 (`KismetMathLibrary.SelectVector` (select `int` _returnvalue_3 :`0` (`self.GetActorForwardVector`) :`1` (`self.GetActorRightVector`) :`2` (`self.GetActorUpVector`)) (select `int` _returnvalue_3 :`0` (1.0 0.0 0.0) :`1` (0.0 1.0 0.0) :`2` (0.0 0.0 1.0) :!type "Vector Structure") (`self.bLocal`))))
  (bind (_returnvalue_x _returnvalue_y _returnvalue_z) (`KismetMathLibrary.BreakVector` (* _returnvalue_5 0.01)))
  (bind (_returnvalue_x_2 _returnvalue_y_2 _returnvalue_z_2) (`KismetMathLibrary.BreakVector` (* _returnvalue_5 1.0)))
  (bind _returnvalue_7 (select `int` _returnvalue_4 :`0` _returnvalue_x_2 :`1` _returnvalue_y_2 :`2` _returnvalue_z_2))
  (bind _returnvalue_8 (select `int` (`KismetStringLibrary.Conv_StringToInt` (`KismetStringLibrary.Conv_NameToString` (`|GetArrayItem` (`ActorComponent.ComponentTags` (`self.ComponentRef`)) 1))) :`0` (`KismetMathLibrary.MakeVector` _returnvalue_x) :`1` (`KismetMathLibrary.MakeVector` 0.0 _returnvalue_y) :`2` (`KismetMathLibrary.MakeVector` 0.0 0.0 _returnvalue_z) :`3` (`KismetMathLibrary.Conv_DoubleToVector` _returnvalue_z)))
  (bind _returnvalue_9 (`KismetMathLibrary.SelectVector` (`KismetMathLibrary.TransformLocation` _returnvalue_2 (`KismetMathLibrary.Vector_SnappedToGrid` (`KismetMathLibrary.InverseTransformLocation` _returnvalue_2 _returnvalue_6) (`self.LocaltionSnapSize`))) _returnvalue_6 (`self.bSnap`)))
  (bind _returnvalue_10 (`KismetMathLibrary.RotatorFromAxisAndAngle` (select `int` _returnvalue_4 :`0` (1.0 0.0 0.0) :`1` (0.0 1.0 0.0) :`2` (0.0 0.0 1.0) :!type "Vector Structure") (`KismetMathLibrary.SelectFloat` (`KismetMathLibrary.GridSnap_Float` _returnvalue_7 (`self.RotationSnapSize`)) _returnvalue_7 (`self.bSnap`))))
  (bind _returnvalue_11 (`KismetMathLibrary.ComposeRotators` (`self.RotationSave`) _returnvalue_10))
  (bind _returnvalue_12 (+ (`self.LocationSave`) _returnvalue_9))
  (bind _returnvalue_13 (+ (`self.ScaleSave`) (`KismetMathLibrary.SelectVector` (`KismetMathLibrary.Vector_SnappedToGrid` _returnvalue_8 (`self.ScaleSnapSize`)) _returnvalue_8 (`self.bSnap`))))
  (bind _z (.z _returnvalue_13))
  (switch `name` (`|GetArrayItem` (`ActorComponent.ComponentTags` (`self.ComponentRef`)))
    (:`location`
      (`self.K2_SetActorLocation` (`self.ActorRef`) _returnvalue_12 false false)
      (`self.K2_SetActorLocation` _returnvalue_12)
      (set `/Visualization/Blueprint/Gizmo/UMG/Gizmo_UI.Text` (`KismetTextLibrary.Conv_DoubleToText` (select `int` (`KismetStringLibrary.Conv_StringToInt` (`KismetStringLibrary.Conv_NameToString` (`|GetArrayItem` (`ActorComponent.ComponentTags` (`self.ComponentRef`)) 1))) :`0` (.x _returnvalue_9) :`1` (.y _returnvalue_9) :`2` (.z _returnvalue_9)) "HalfToEven") (`self.UI_Ref`)))
    (:`rotation`
      (`self.K2_SetActorRotation` (`self.ActorRef`) _returnvalue_11 false)
      (if (`self.bLocal`)
        (`self.K2_SetActorRotation` _returnvalue_11))
      (set `/Visualization/Blueprint/Gizmo/UMG/Gizmo_UI.Text` (`KismetTextLibrary.Conv_DoubleToText` (select `int` (`KismetStringLibrary.Conv_StringToInt` (`KismetStringLibrary.Conv_NameToString` (`|GetArrayItem` (`ActorComponent.ComponentTags` (`self.ComponentRef`)) 1))) :`0` (.roll _returnvalue_10) :`1` (.pitch _returnvalue_10) :`2` (.yaw _returnvalue_10)) "HalfToEven") (`self.UI_Ref`)))
    (:`scale`
      (`self.SetActorScale3D` (`self.ActorRef`) _returnvalue_13)
      (set `/Visualization/Blueprint/Gizmo/UMG/Gizmo_UI.Text` (`KismetTextLibrary.Conv_DoubleToText` (select `int` (`KismetStringLibrary.Conv_StringToInt` (`KismetStringLibrary.Conv_NameToString` (`|GetArrayItem` (`ActorComponent.ComponentTags` (`self.ComponentRef`)) 1))) :`0` (.x _returnvalue_13) :`1` (.y _returnvalue_13) :`2` _z :`3` _z) "HalfToEven") (`self.UI_Ref`)))))

(fn `GizmoReady`
  (params (Hit :type "HitResult Structure"))
  (bind (_bblockinghit _binitialoverlap _time _distance _location _impactpoint _normal _impactnormal _physmat _hitactor _hitcomponent) (`GameplayStatics.BreakHitResult` Hit))
  (bind _returnvalue (`GameplayStatics.GetPlayerController` 0))
  (bind _componentref (`self.ComponentRef`))
  (bind _componentref_2 (`self.ComponentRef`))
  (bind (_returnvalue_location _returnvalue_rotation _returnvalue_scale) (`KismetMathLibrary.BreakTransform` (`self.GetTransform` (`self.ActorRef`))))
  (bind (_locationx _locationy) (`PlayerController.GetMousePosition` _returnvalue))
  (bind (_worldposition _worlddirection) (`GameplayStatics.DeprojectScreenToWorld` _returnvalue (`KismetMathLibrary.MakeVector2D` _locationx _locationy)))
  (if (!= self _hitactor)
    ;[1 1 1] 保存交互物体并做交互准备
    (set `self.ActorRef` _hitactor) ; 保存交互物体
    (`self.SetActorHiddenInGame` false) ; 显示坐标
    (`self.K2_SetActorLocation` (`self.K2_GetActorLocation` (`self.ActorRef`))) ; 坐标位置与交互物体重合
    ;[1 1 1] 重置选中组件
    (`/Engine/EditorBlueprintResources/StandardMacros.IsValid` _componentref_2
      (:`Is Valid`
        (bind _returnvalue_2 (`PrimitiveComponent.CreateDynamicMaterialInstance` _componentref_2 0 null "None"))
        (`MaterialInstanceDynamic.SetScalarParameterValue` _returnvalue_2 "intensity" 1.0)))
    (else
      ;[1 1 1] 更改选中组件
      (`/Engine/EditorBlueprintResources/StandardMacros.IsValid` _componentref
        (:`Is Valid`
          (bind _returnvalue_3 (`PrimitiveComponent.CreateDynamicMaterialInstance` _componentref 0 null "None"))
          (`MaterialInstanceDynamic.SetScalarParameterValue` _returnvalue_3 "intensity" 1.0))
        (:`Is Not Valid`
          _))
      (bind _output_get (set `self.ComponentRef` _hitcomponent)) ; 通过被点击组件tag设置交互方式
      (bind _returnvalue_4 (`PrimitiveComponent.CreateDynamicMaterialInstance` _output_get 0 null "None"))
      (`MaterialInstanceDynamic.SetScalarParameterValue` _returnvalue_4 "intensity" 10.0)
      ;[1 1 1] 按坐标轴不同组件做相应具体准备
      (set `self.LocationSave` _returnvalue_location) ; 位置
      (set `self.RotationSave` _returnvalue_rotation) ; 旋转
      (set `self.ScaleSave` _returnvalue_scale) ; 缩放
      (set `self.VirtualPlaneSave` (`KismetMathLibrary.MakePlaneFromPointAndNormal` (`self.K2_GetActorLocation`) (select `int` (`KismetStringLibrary.Conv_StringToInt` (`KismetStringLibrary.Conv_NameToString` (`|GetArrayItem` (`ActorComponent.ComponentTags` (`self.ComponentRef`)) 1))) :`0` (0.0 0.0 1.0) :`1` (0.0 0.0 1.0) :`2` (1.0 0.0 0.0) :`3` (`self.GetActorForwardVector` (`GameplayStatics.GetPlayerCameraManager` 0))))) ; 创建虚拟平面
      (set `self.VirtualPositionSave` (`.Intersection` (`KismetMathLibrary.LinePlaneIntersection` _worldposition (+ _worldposition (* _worlddirection (`PlayerController.HitResultTraceDistance` _returnvalue))) (`self.VirtualPlaneSave`)))) ; 保存鼠标在虚拟平面上的点
      ;[1 1 1] 设置坐标旋转
      (if (`self.bLocal`)
        (`self.K2_SetActorRotation` (`self.K2_GetActorRotation` (`self.ActorRef`)) :!label _label) ; 坐标旋转与交互物体重合
        (else
          (switch `name` (`|GetArrayItem` (`ActorComponent.ComponentTags` (`self.ComponentRef`)))
            (:`location`
              _)
            (:`rotation`
              _)
            (:`scale`
              (goto _label)))
          (`self.K2_SetActorRotation` (struct)))))))

(fn `GizmoSize`
  (`self.SetActorScale3D` (`KismetMathLibrary.Conv_DoubleToVector` (/ (`KismetMathLibrary.Vector_Distance` (`PlayerCameraManager.GetCameraLocation` (`GameplayStatics.GetPlayerCameraManager` 0)) (`self.K2_GetActorLocation`)) (`self.GizmoSizeValue`)))))

(fn `UserConstructionScript`
  (`MeshComponent.SetVectorParameterValueOnMaterials` (`self.Locat_X`) "color" (1.0 0.0 0.0))
  (`MeshComponent.SetVectorParameterValueOnMaterials` (`self.Rotat_X`) "color" (1.0 0.0 0.0))
  (`MeshComponent.SetVectorParameterValueOnMaterials` (`self.Scale_X`) "color" (1.0 0.0 0.0)) ; X
  (`MeshComponent.SetVectorParameterValueOnMaterials` (`self.Locat_Y`) "color" (0.0 1.0 0.0))
  (`MeshComponent.SetVectorParameterValueOnMaterials` (`self.Rotat_Y`) "color" (0.0 1.0 0.0))
  (`MeshComponent.SetVectorParameterValueOnMaterials` (`self.Scale_Y`) "color" (0.0 1.0 0.0)) ; Y
  (`MeshComponent.SetVectorParameterValueOnMaterials` (`self.Locat_Z`) "color" (0.0 0.0 1.0))
  (`MeshComponent.SetVectorParameterValueOnMaterials` (`self.Rotat_Z`) "color" (0.0 0.0 1.0))
  (`MeshComponent.SetVectorParameterValueOnMaterials` (`self.Scale_Z`) "color" (0.0 0.0 1.0)) ; Z
)