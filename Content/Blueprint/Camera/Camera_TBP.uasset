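; Roaming camera actor that moves a camera along a spline, facing along the path or at a target, for idle and birdeye views.
; A timeline steps the spline position each update, looping or stopping at the end.
; Looping timers compare mouse position to start roaming when it is idle and blend back to the pawn when it moves.
; A birdeye event either starts roaming or, with UsePawn, slowly yaws the player's control rotation.
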(event `self.ReceiveBeginPlay`
  ;[1 1 1] 开始
  (add `/Visualization/GamePlay/VGIS.Birdeye_ED` (subsystem `/Visualization/GamePlay/VGIS`) (`|CreateDelegate` :!event `Birdeye_Event`))
  (`|ExecutionSequence`
    (:`then_0`
      (if (`self.bBeginRoaming`)
        (`self.Roaming_Event`)))
    (:`then_1`
      (if (`self.bBeginCheckRoaming`)
        (`self.CheckRoaming_Event`)))))

(event `Play_Event`
  ;[0.3 1 0] 相机移动
  (`Timeline|Timeline_Move` :!label _label
    (:`Update`
      (`self.MoveCamera` (`self.TimeOfSpline`) (`self.AddPosition`))
      (`self.IsMoveEnd`))))

(event `Stop_Event`
  ;[0.3 1 0] 相机移动
  (goto _label :!via `Stop`))

(event `Roaming_Event`
  ;[0.3 1 0 0.3] 开始漫游
  (`PlayerController.SetViewTargetWithBlend` (`GameplayStatics.GetPlayerController` 0) self 1.0 "VTBlend_Linear" 0.0 false)
  (`self.Play_Event`))

(event `CheckRoaming_Event`
  ;[0.3 1 0 0.3] 漫游检测
  (bind _returnvalue (`KismetSystemLibrary.K2_SetTimer` null "CheckRoaming" (`self.CheckRoamingTime`) true))
  (set `self.CheckRoaming_Timer` _returnvalue))

(event `NotRoaming`
  ;[1 0.3 0 0.3] 停止漫游
  (`PlayerController.SetViewTargetWithBlend` (`GameplayStatics.GetPlayerController` 0) (`GameplayStatics.GetPlayerPawn` 0) 1.0 "VTBlend_Linear" 0.0 false)
  (`self.Stop_Event`))

(event `StopCheckRoaming_Event`
  ;[1 0.3 0 0.3] 停止漫游检测
  (`self.NotRoaming`)
  (`KismetSystemLibrary.K2_ClearAndInvalidateTimerHandle` (`self.CheckRoaming_Timer`))
  (`KismetSystemLibrary.K2_ClearAndInvalidateTimerHandle` (`self.CheckNotRoaming_Timer`)))

(event `Birdeye_Event`
  (params (bBirdeye :type Boolean))
  (bind _returnvalue (`GameplayStatics.GetPlayerController` 0))
  (bind _busepawn (`self.bUsePawn`))
  ;[1 0 0] 鸟瞰事件
  (if bBirdeye
    (if _busepawn
      (`Timeline|Timeline_0` :!label _label
        (:`Update`
          (`Controller.SetControlRotation` _returnvalue (`KismetMathLibrary.MakeRotator` (.roll (`Controller.GetControlRotation` _returnvalue)) (.pitch (`Controller.GetControlRotation` _returnvalue)) (+ (.yaw (`Controller.GetControlRotation` _returnvalue)) 0.1)))))
      (else
        (`self.Roaming_Event`)))
    (elif _busepawn
      (goto _label :!via `Stop`)
      (else
        (`self.NotRoaming`)))))

(fn `CheckNotRoaming`
  (bind _returnvalue (`WidgetLayoutLibrary.GetMousePositionOnViewport`))
  (if (`KismetMathLibrary.NotEqualExactly_Vector2DVector2D` _returnvalue (`self.MousePisotion`))
    (`self.NotRoaming`)
    (`KismetSystemLibrary.K2_PauseTimerHandle` (`self.CheckNotRoaming_Timer`))
    (`KismetSystemLibrary.K2_UnPauseTimerHandle` (`self.CheckRoaming_Timer`))))

(fn `CheckRoaming`
  (bind _returnvalue (`WidgetLayoutLibrary.GetMousePositionOnViewport`))
  (if (`KismetMathLibrary.EqualExactly_Vector2DVector2D` _returnvalue (`self.MousePisotion`))
    (`self.Roaming_Event`)
    (`KismetSystemLibrary.K2_PauseTimerHandle` (`self.CheckRoaming_Timer`))
    (bind _returnvalue_2 (`KismetSystemLibrary.K2_SetTimer` null "CheckNotRoaming" 0.02 true))
    (set `self.CheckNotRoaming_Timer` _returnvalue_2)
    (else
      (set `self.MousePisotion` _returnvalue))))

(fn `IsMoveEnd`
  (if (>= (`self.TimeOfSpline`) 1.0)
    (if (`self.bViewLoop`)
      (set `self.TimeOfSpline` 0.0)
      (else
        (`self.Stop_Event`)))))

(fn `MoveCamera`
  (params (PositionOnRail :type "Float (double-precision)") (AddPosition :type "Float (double-precision)"))
  (bind _camerapath (`self.CameraPath`))
  (bind _output_get (set `self.TimeOfSpline` (+ PositionOnRail AddPosition)))
  (`SceneComponent.K2_SetWorldLocation` (`self.Camera`) (`SplineComponent.GetLocationAtTime` _camerapath _output_get "World" true) false true)
  (if (`self.bAim`)
    (`SceneComponent.K2_SetWorldRotation` (`self.Camera`) (`KismetMathLibrary.FindLookAtRotation` (`SceneComponent.K2_GetComponentLocation` (`self.Camera`)) (`self.K2_GetActorLocation` (select `bool` (`KismetSystemLibrary.IsValid` (`self.AimActor`)) :`false` self :`true` (`self.AimActor`) :!type "Actor Object Reference"))) false false)
    (else
      (`SceneComponent.K2_SetWorldRotation` (`self.Camera`) (`KismetMathLibrary.Conv_VectorToRotator` (`SplineComponent.GetTangentAtTime` _camerapath _output_get "World" true)) false true))))

(fn `Play_SF`
  (`self.Play_Event`))

(fn `Stop_SF`
  (`self.Stop_Event`))

(fn `UserConstructionScript`
  ;[1 1 1] 相机机跟随样条线
  (`self.MoveCamera` (`self.TimeOfSpline`))
  ;[1 1 1] 样条线闭合
  (`SplineComponent.SetClosedLoop` (`self.CameraPath`) (`self.bClosedPath`) true))